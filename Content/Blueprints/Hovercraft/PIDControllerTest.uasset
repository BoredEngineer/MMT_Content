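; Test actor in the Hovercraft folder that uses a PID controller to turn a physics mesh toward a player-steered yaw.
; The LeftRight axis shifts the desired yaw, which an arrow component displays.
; Each tick, the yaw difference between arrow and mesh feeds the PIDController, whose control coefficient is scaled into Z torque on the mesh.
; The coefficient is also drawn as debug text at the actor.
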(event EventBeginPlay)

(event EventActorBeginOverlap
  (params (OtherActor :type Actor%20Object%20Reference)))

(event EventTick
  (params (DeltaSeconds :type Float%20%28single-precision%29))
  (Transformation|SetWorldRotation (Variables|Default|GetArrow) (Variables|Default|GetDesiredRotation) false false)
  (Default|AddMeasuredError (Variables|Default|GetPIDController) (Utilities|Struct|MakeErrorStruct (.yaw (Math|Rotator|Delta(Rotator) (Transformation|GetWorldRotation (Variables|Default|GetArrow)) (Transformation|GetWorldRotation (Variables|Default|GetStaticMesh)))) DeltaSeconds))
  (bind _controlcoefficient (Default|GetControlCoefficient (Variables|Default|GetPIDController)))
  (Rendering|Debug|DrawDebugString (Transformation|GetActorLocation) (Utilities|String|ToString(Float) _controlcoefficient) 0 "(R=1.000000,G=1.000000,B=1.000000,A=1.000000)")
  (Class|PrimitiveComponent|AddTorque (Variables|Default|GetStaticMesh) (Math|Vector|MakeVector 0.0 0.0 (* _controlcoefficient 2e+03)) "None" false))

(event Input|AxisEvents|InputAxisLeftRight
  (params (AxisValue :type Float%20%28single-precision%29))
  (Variables|Default|SetDesiredRotation (Math|Rotator|MakeRotator (.roll (Variables|Default|GetDesiredRotation)) (.pitch (Variables|Default|GetDesiredRotation)) (+ (.yaw (Variables|Default|GetDesiredRotation)) (* AxisValue -0.5)))))

(fn ConstructionScript)