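; MMTFunctionLibrary is a set of shared helper functions for components to query their owning actor.
; Two lookups scan the owner's components and return the mesh or scene component whose object name matches a given name, with MeshComponent covering both static and skeletal meshes.
; A third check reports whether the owner implements PSSVisualDebuggerInterface, printing an on-screen warning when it does not.
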(fn GetMeshComponentReferencebyName
  (params (Target :type Scene%20Component%20Object%20Reference) (ComponentName :type String))
  (for _array_element (Actor|GetComponentsByClass (Components|GetOwner Target) "/Script/Engine.MeshComponent")
    (if (Utilities|Enum|Equal(Enum) (Utilities|GetObjectName _array_element) ComponentName)
      (LocalVariables|SetLocComponentRef _array_element)))
  (return (LocalVariables|GetLocComponentRef)))

(fn CheckParentforVisualDebugComponent
  (params (Target :type Scene%20Component%20Object%20Reference))
  (bind _returnvalue (Components|GetOwner Target))
  (if (Utilities|DoesObjectImplementInterface _returnvalue "/Game/Blueprints/ReUsableComponents/PhysicsSubSteppingVisualDebugger/PSSVisualDebuggerInterface.PSSVisualDebuggerInterface_C")
    (LocalVariables|SetLocAvailable true)
    (else
      (LocalVariables|SetLocAvailable false)
      (Development|PrintString 0 (Utilities|String|Append (Utilities|GetObjectName _returnvalue) "->" (Utilities|GetObjectName Target) "->" "Debug is enabled but owner doesn't support PSS Visual Debugging") true true "(R=1.000000,G=0.000000,B=0.064224,A=1.000000)" 1e+01)))
  (return (LocalVariables|GetLocAvailable)))

(fn GetSceneComponentReferencebyName
  (params (Target :type Scene%20Component%20Object%20Reference) (ComponentName :type String))
  (for _array_element (Actor|GetComponentsByClass (Components|GetOwner Target) "/Script/Engine.SceneComponent")
    (if (Utilities|Enum|Equal(Enum) (Utilities|GetObjectName _array_element) ComponentName)
      (LocalVariables|SetLocComponentRef _array_element)))
  (return (LocalVariables|GetLocComponentRef)))