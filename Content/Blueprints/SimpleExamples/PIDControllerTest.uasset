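; PIDControllerTest is a possessable example that demonstrates a PID controller turning a mesh to follow a target heading.
; The right/left input axis changes a desired yaw, which is applied to an arrow each tick.
; The yaw difference between arrow and mesh feeds the PID controller, whose control coefficient is scaled into yaw torque on the mesh.
; A help sign shows possession or rotation key hints.
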(event EventPossessed
  (params (NewController :type Controller%20Object%20Reference))
  (Rendering|Components|TextRender|SetText (Variables|Default|GetHelpSign) (Utilities|Text|MakeLiteralText "Press A/D to rotate")))

(event EventUnpossessed
  (params (OldController :type Controller%20Object%20Reference))
  (Rendering|Components|TextRender|SetText (Variables|Default|GetHelpSign) (Utilities|Text|MakeLiteralText "Press 2 to posses")))

(event EventBeginPlay)

(event EventActorBeginOverlap
  (params (OtherActor :type Actor%20Object%20Reference)))

(event EventTick
  (params (DeltaSeconds :type Float%20%28single-precision%29))
  (Transformation|SetWorldRotation (Variables|Default|GetArrow) (Variables|Default|GetDesiredRotation) false false)
  (Default|AddMeasuredError (Variables|Default|GetPIDController) (Utilities|Struct|MakePIDErrorStruct (.yaw (Math|Rotator|Delta(Rotator) (Transformation|GetWorldRotation (Variables|Default|GetArrow)) (Transformation|GetWorldRotation (Variables|Default|GetStaticMesh)))) DeltaSeconds))
  (bind _controlcoefficient (Default|GetControlCoefficient (Variables|Default|GetPIDController)))
  (Class|PrimitiveComponent|AddTorque (Variables|Default|GetStaticMesh) (Math|Vector|MakeVector 0.0 0.0 (* _controlcoefficient 2e+03)) "None" false))

(event Input|AxisEvents|InputAxisVehicleRightLeft
  (params (AxisValue :type Float%20%28single-precision%29))
  (Variables|Default|SetDesiredRotation (Math|Rotator|MakeRotator (.roll (Variables|Default|GetDesiredRotation)) (.pitch (Variables|Default|GetDesiredRotation)) (+ (.yaw (Variables|Default|GetDesiredRotation)) (* AxisValue 0.5)))))

(fn ConstructionScript
  (Rendering|Components|TextRender|SetText (Variables|Default|GetHelpSign) (Utilities|Text|MakeLiteralText "Press 2 to posses")))