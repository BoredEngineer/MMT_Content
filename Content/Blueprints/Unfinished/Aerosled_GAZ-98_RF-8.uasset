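; Unfinished Aerosled GAZ-98 RF-8 vehicle Blueprint with basic physics and camera controls.
; Four corner suspension components receive PhysicsUpdate from the MMTPhysicsTick substep event.
; The F key applies a mass-independent forward impulse to the root on each press, with no steering or continuous thrust in the graph.
; Zoom inputs shorten or lengthen the spring arm in fixed, unclamped steps.
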(event EventBeginPlay)

(event EventActorBeginOverlap
  (params (OtherActor :type Actor%20Object%20Reference)))

(event EventMMTPhysicsTick
  (params (SubstepDeltaTime :type Float%20%28single-precision%29))
  (Default|PhysicsUpdate (Variables|Default|GetSuspFR) SubstepDeltaTime))

(event EventTick
  (params (DeltaSeconds :type Float%20%28single-precision%29)))

(event Input|ActionEvents|InputActionZoomIn
  (params (Key :type Key%20Structure :default "AnyKey"))
  (bind _springarm (Variables|Default|GetSpringArm))
  ;[1 1 1] Camera Control
  (:Pressed
    (Variables|/Script/Engine.SpringArmComponent|SetTargetArmLength _springarm (+ (Variables|/Script/Engine.SpringArmComponent|GetTargetArmLength _springarm) -25.0))))

(event Input|ActionEvents|InputActionZoomOut
  (params (Key :type Key%20Structure :default "AnyKey"))
  (bind _springarm (Variables|Default|GetSpringArm))
  ;[1 1 1] Camera Control
  (:Pressed
    (Variables|/Script/Engine.SpringArmComponent|SetTargetArmLength _springarm (+ (Variables|/Script/Engine.SpringArmComponent|GetTargetArmLength _springarm) 25.0))))

(event Input|KeyboardEvents|F
  (params (Key :type Key%20Structure :default "AnyKey"))
  (:Pressed
    (Physics|AddImpulse (Variables|Default|GetRoot) (* (Transformation|GetActorForwardVector) 1e+02) "None" true)))

(fn ConstructionScript)