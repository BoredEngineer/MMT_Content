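; An unfinished-folder physics demo pawn: a possessable ball, held by top and bottom spring components, that the player punches.
; MMTPhysicsTick updates both springs with the substep delta time.
; Left click applies a randomly scaled force to the ball along the camera-to-ball direction.
; Zoom inputs change the spring arm length, and a help sign switches between possess and punch prompts with possession.
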(event EventPossessed
  (params (NewController :type Controller%20Object%20Reference))
  (Rendering|Components|TextRender|SetText (Variables|Default|GetHelpSign) (Utilities|Text|MakeLiteralText "Left Click to punch")))

(event EventUnpossessed
  (params (OldController :type Controller%20Object%20Reference))
  (Rendering|Components|TextRender|SetText (Variables|Default|GetHelpSign) (Utilities|Text|MakeLiteralText "Press 1 to posses")))

(event EventBeginPlay)

(event EventActorBeginOverlap
  (params (OtherActor :type Actor%20Object%20Reference)))

(event EventTick
  (params (DeltaSeconds :type Float%20%28single-precision%29)))

(event EventMMTPhysicsTick
  (params (SubstepDeltaTime :type Float%20%28single-precision%29))
  (Default|PhysicsUpdate (Variables|Default|GetTopPhysSpring) SubstepDeltaTime))

(event Input|ActionEvents|InputActionZoomIn
  (params (Key :type Key%20Structure :default "AnyKey"))
  (bind _springarm (Variables|Default|GetSpringArm))
  ;[1 1 1] Camera Control
  (:Pressed
    (Variables|/Script/Engine.SpringArmComponent|SetTargetArmLength _springarm (+ (Variables|/Script/Engine.SpringArmComponent|GetTargetArmLength _springarm) -25.0))))

(event Input|ActionEvents|InputActionZoomOut
  (params (Key :type Key%20Structure :default "AnyKey"))
  (bind _springarm (Variables|Default|GetSpringArm))
  ;[1 1 1] Camera Control
  (:Pressed
    (Variables|/Script/Engine.SpringArmComponent|SetTargetArmLength _springarm (+ (Variables|/Script/Engine.SpringArmComponent|GetTargetArmLength _springarm) 25.0))))

(event Input|MouseEvents|LeftMouseButton
  (params (Key :type Key%20Structure :default "AnyKey"))
  (:Pressed
    (Physics|AddForce (Variables|Default|GetBall) (* (Math|Vector|Normalize (- (Transformation|GetWorldLocation (Variables|Default|GetBall)) (Transformation|GetWorldLocation (Variables|Default|GetCamera)))) (Math|Random|RandomFloatinRange 5e+05 7.5e+05)) "None" false)))

(fn ConstructionScript
  (Rendering|Components|TextRender|SetText (Variables|Default|GetHelpSign) (Utilities|Text|MakeLiteralText "Press 1 to posses")))