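; Propeller engine component that pushes a chassis with force applied at its own location, along the propeller's forward vector.
; On BeginPlay it finds chassis and propeller by component name, logging missing references.
; Each tick, throttle ramps up at half its fall rate and drives curve-scaled thrust, with input sign setting direction and zero input cutting force immediately.
; Propeller spin follows throttle, even in sleep mode, which skips thrust updates and force.
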(event EventBeginPlay
  (CallFunction|GetComponentsReference))

(event EventTick
  (params (DeltaSeconds :type Float%20%28single-precision%29))
  (CallFunction|AnimatePropeller)
  (if (Variables|Default|GetSleepMod)
    (if (Variables|Default|GetDebug?)
      (Rendering|Debug|DrawDebugString (Transformation|GetWorldLocation) "Sleeping..." 0 "(R=1.000000,G=1.000000,B=1.000000,A=1.000000)"))
    (else
      (CallFunction|UpdateThrust)
      (CallFunction|ApplyThrust))))

(fn GetComponentsReference
  (Utilities|FlowControl|Sequence
    (:then_0
      (bind _componentref (Utilities|GetComponentReferencebyName self (Variables|Default|GetChasisComponentName)) ; Macro to find component by name in the same blueprint
        (:InLoopExecution!
          (Variables|Components|SetChassis _componentref))))
    (:then_1
      (bind _componentref_2 (Utilities|GetComponentReferencebyName self (Variables|Default|GetPropellerMeshName)) ; Macro to find component by name in the same blueprint
        (:InLoopExecution!
          (Variables|Components|SetPropeller _componentref_2))))
    (:then_2
      (Utilities|IsValid (Variables|Components|GetChassis)
        (:Is%20Not%20Valid
          (Utilities|LogErrorReferencebyName self (Variables|Default|GetChasisComponentName)) ; Macro to throw error into log
        )))
    (:then_3
      (Utilities|IsValid (Variables|Components|GetPropeller)
        (:Is%20Not%20Valid
          (Utilities|LogErrorReferencebyName self (Variables|Default|GetPropellerMeshName)) ; Macro to throw error into log
        )))))

(fn ApplyThrust
  (Class|PrimitiveComponent|AddForceatLocation (Variables|Components|GetChassis) (Variables|Default|GetThrustForce) (Transformation|GetWorldLocation) "None"))

(fn UpdateThrust
  (bind _propeller (Variables|Components|GetPropeller))
  (bind _returnvalue (Transformation|GetWorldLocation _propeller))
  (Variables|Default|SetEngineThrottle (Math|Float|Clamp(Float) (+ (Variables|Default|GetEngineThrottle) (* (Math|Float|SelectFloat 0.5 -1.0 (!= (Variables|Default|GetInputThrottle) 0.0)) (Utilities|Time|GetWorldDeltaSeconds)))))
  (Variables|Default|SetThrustForce (* (* (Math|Vector|GetForwardVector (Variables|Components|GetPropeller)) (Math|Float|Sign(Float) (Variables|Default|GetInputThrottle))) (* (Math|Curves|GetFloatValue (Variables|Default|GetThrottleCurve) (Variables|Default|GetEngineThrottle)) (Variables|Default|GetThrusterMaxForce))))
  (if (Variables|Default|GetDebug?)
    (Rendering|Debug|DrawDebugLine :LineStart _returnvalue :LineEnd (+ _returnvalue (* (* (Math|Vector|GetForwardVector (Variables|Components|GetPropeller)) (Math|Float|Sign(Float) (Variables|Default|GetInputThrottle))) (* (Math|Curves|GetFloatValue (Variables|Default|GetThrottleCurve) (Variables|Default|GetEngineThrottle)) (Variables|Default|GetThrusterMaxForce)))) :Thickness 5.0)
    (Rendering|Debug|DrawDebugString (Transformation|GetWorldLocation) (Utilities|String|Append "Throttle: " (Utilities|String|ToString(Float) (Variables|Default|GetEngineThrottle))) 0 "(R=1.000000,G=1.000000,B=1.000000,A=1.000000)")))

(fn SetThrottle
  (params (Throttle :type Float%20%28single-precision%29))
  (Variables|Default|SetInputThrottle Throttle)
  (return false))

(fn AnimatePropeller
  (Transformation|AddLocalRotation (Variables|Components|GetPropeller) (Math|Rotator|MakeRotator (* (Math|Float|Lerp (Variables|Default|GetMinPropVelocity) (Variables|Default|GetMaxPropVelocity) (Variables|Default|GetEngineThrottle)) -1.0) 0.0 0.0) false false))

(fn SwitchSleepMod
  (params (SleepMod :type Boolean))
  (Variables|Default|SetSleepMod SleepMod)
  (return false))