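; PID controller component that turns a stream of measured errors into a control coefficient.
; AddMeasuredError keeps a capped, newest-first history of error values with their delta times, which ResetController clears.
; GetControlCoefficient sums weighted proportional, integral and derivative terms: the latest error, a time-weighted sum over the stored history, and the rate between the last two samples.
; The terms are only computed once at least two samples are stored.
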(event EventBeginPlay)

(event EventTick
  (params (DeltaSeconds :type Float%20%28single-precision%29)))

(fn AddMeasuredError
  (params (MeasuredError :type Error%20Struct%20Structure))
  (bind _measurederrors (Variables|Default|GetMeasuredErrors))
  (Utilities|Array|Insert (Variables|Default|GetMeasuredErrors) MeasuredError)
  ;[1 1 1] Remove last element if we have enough errors to work with
  (if (> (Utilities|Array|Length (Variables|Default|GetMeasuredErrors)) (Variables|Default|GetNumOfErrorsToStore))
    (Utilities|Array|RemoveIndex _measurederrors (Utilities|Array|LastIndex _measurederrors))))

(fn GetControlCoefficient
  (bind _measurederrors (Variables|Default|GetMeasuredErrors))
  (bind _item (Utilities|Array|Get(acopy) _measurederrors))
  (if (>= (Utilities|Array|Length (Variables|Default|GetMeasuredErrors)) 2)
    ;[1 1 1] Proportional error is the last measured error
    (LocalVariables|SetProportionalError (.measuredvalue (Utilities|Array|Get(acopy) (Variables|Default|GetMeasuredErrors))))
    ;[1 1 1] Integral error is integrated over N last measurements taking into account delta time
    (for _array_element (Variables|Default|GetMeasuredErrors)
      (LocalVariables|SetIntegralError (+ (LocalVariables|GetIntegralError) (* (.measuredvalue _array_element) (.deltatime _array_element)))))
    ;[1 1 1] Derivative is a difference between last two measured errors divided by time between them
    (LocalVariables|SetDerivativeError (/ (- (.measuredvalue _item) (.measuredvalue (Utilities|Array|Get(acopy) _measurederrors 1))) (.deltatime _item))))
  (return (+ (* (Variables|Default|GetProportionalCoefficient) (LocalVariables|GetProportionalError)) (* (Variables|Default|GetIntegralCoefficient) (LocalVariables|GetIntegralError)) (* (Variables|Default|GetDerivativeCoefficient) (LocalVariables|GetDerivativeError)))))

(fn ResetController
  (Utilities|Array|Clear (Variables|Default|GetMeasuredErrors)))