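; Hovercraft thruster component that simulates an air cushion pushing the chassis up from the component's location.
; A downward sphere trace measures ground distance, turning eased engine throttle into inverse-square pressure that fades once the gap exceeds the skirt.
; A velocity-based damping term counters spring oscillation, and the trace also sets the skirt end position.
; Tick only eases throttle; force calculation and application are separate functions not called here.
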(event EventBeginPlay
  (CallFunction|GetComponentsReference))

(event EventTick
  (params (DeltaSeconds :type Float%20%28single-precision%29))
  (CallFunction|UpdateThrottle))

(fn GetComponentsReference
  (Utilities|FlowControl|Sequence
    (:then_0
      (bind _componentref (Utilities|GetComponentReferencebyName self (Variables|Default|GetChasisComponentName)) ; Macro to find component by name in the same blueprint
        (:InLoopExecution!
          (Variables|Components|SetChassis _componentref))))
    (:then_1
      (Utilities|IsValid (Variables|Components|GetChassis)
        (:Is%20Not%20Valid
          (Utilities|LogErrorReferencebyName self (Variables|Default|GetChasisComponentName)) ; Macro to throw error into log
        )))))

(fn CalculateAirPressureForce
  (params (DeltaTime :type Float%20%28single-precision%29))
  (bind _returnvalue (Math|Vector|GetUpVector))
  (bind _returnvalue_2 (Transformation|GetWorldLocation))
  (bind _spheretraceradius (Variables|Default|GetSphereTraceRadius))
  (bind _distancetoskirtedge (Variables|Default|GetDistanceToSkirtEdge))
  (bind _returnvalue_3 (* _returnvalue _spheretraceradius))
  (bind _returnvalue_4 (+ _returnvalue_2 _returnvalue_3))
  (bind _outhit (Class|KismetSystemLibrary|SphereTraceSingleNEW _returnvalue_4 (+ _returnvalue_2 (* (Math|Vector|GetUpVector) (* (+ (Variables|Default|GetDistanceToSkirtEdge) (Variables|Default|GetMaxDistanceBeyoundSkirtEdge)) -1.0))) (Variables|Default|GetSphereTraceRadius) "TraceTypeQuery1" false (Utilities|Array|MakeArray (Components|GetOwner)) "ForOneFrame" true))
  (if (.bblockinghit _outhit)
    (bind _output_get (LocalVariables|SetActualDistance (Math|Vector|VectorLength (- (.location _outhit) _returnvalue_4))))
    (Rendering|Debug|DrawDebugString (Transformation|GetWorldLocation) (Utilities|String|ToString(Float) _output_get) 0 "(R=1.000000,G=1.000000,B=1.000000,A=1.000000)")
    (LocalVariables|SetMaximumForce (* (Variables|Default|GetEngineThrottle) (Variables|Default|GetThrusterMaxForce)))
    (Math|Float|CompareFloat (LocalVariables|GetActualDistance) (Variables|Default|GetDistanceToSkirtEdge)
      (:>
        ;[1 1 1] If there is a gap between ground and the skirt we will loose some air pressure until
        ; the gap is too big to maintan any usable pressure
        (Variables|Default|SetTargetAirPressure (Math|Float|Lerp (/ (LocalVariables|GetMaximumForce) (* _distancetoskirtedge _distancetoskirtedge)) 0.0 (/ (- (LocalVariables|GetActualDistance) (Variables|Default|GetDistanceToSkirtEdge)) (Variables|Default|GetMaxDistanceBeyoundSkirtEdge))))
        (CallFunction|SetSkirtEndPosition (Variables|Default|GetDistanceToSkirtEdge) :!label _label) ; If ground is furter than skirt edge than pin it to maximum skirt length
      )
      (:==
        ;[1 1 1] Skirt is touching the ground, air pressure is proportional to volume of air
        ; and force of the engine. Pressure of liquids normally has a qudratic distribution
        ; so we take a square of the length as aproximation to volume.
        (Variables|Default|SetTargetAirPressure (/ (LocalVariables|GetMaximumForce) (* (LocalVariables|GetActualDistance) (LocalVariables|GetActualDistance))) :!label _label_2)
        (CallFunction|SetSkirtEndPosition (LocalVariables|GetActualDistance)))
      (:<
        (goto _label_2)))
    (else
      (Variables|Default|SetTargetAirPressure 0.0) ; If distance is too large, air cussion effect is lost
      (goto _label)))
  (Variables|Default|SetAirPressureForce (* (Math|Vector|GetUpVector) (+ (Variables|Default|GetTargetAirPressure) (|(A*(B-C)) (Variables|Default|GetDampingCoefficient) 0.0 (/ (- (LocalVariables|GetActualDistance) (Variables|Default|GetPreviousActualDistance)) DeltaTime)))))
  (Variables|Default|SetPreviousActualDistance (LocalVariables|GetActualDistance))
  (return (Variables|Default|GetAirPressureForce)))

(fn UpdateThrottle
  (Variables|Default|SetEngineThrottle (Math|Interpolation|FInterptoConstant (Variables|Default|GetEngineThrottle) (Variables|Default|GetInputThrottle) (Utilities|Time|GetWorldDeltaSeconds) 0.2)))

(fn SetThrottle
  (params (Throttle :type Float%20%28single-precision%29))
  (Variables|Default|SetInputThrottle Throttle)
  (return false))

(fn GetSkirtEndPosition
  (return (Variables|Default|GetSkirtEndPosition)))

(fn SetSkirtEndPosition
  (params (MeasuredDistance :type Float%20%28single-precision%29))
  (Variables|Default|SetSkirtEndPosition (+ (Transformation|GetWorldLocation) (* (Math|Vector|GetUpVector) (* MeasuredDistance -1.0)))))

(fn ApplyAirPressureForce
  (params (PercentOfForceToApply :type Float%20%28single-precision%29))
  (Class|PrimitiveComponent|AddForceatLocation (Variables|Components|GetChassis) (* (Variables|Default|GetAirPressureForce) PercentOfForceToApply) (Transformation|GetWorldLocation) "None"))

(fn SwitchSleepMod
  (params (SleepMod :type Boolean))
  (Variables|Default|SetSleepMod SleepMod)
  (return false))