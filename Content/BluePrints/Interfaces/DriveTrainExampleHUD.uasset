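; Blueprint interface through which a drivetrain example HUD reads engine and clutch state.
; It declares getters for engine RPM with a display color, throttle, torque, clutch status text and ignition state.
; The functions here return only empty defaults, leaving the actual values to whichever class implements the interface.
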(fn HUDGetEngineRPM
  (return 0.0))

(fn HUDGetThrottle
  (return 0.0))

(fn HUDGetEngineTorque
  (return 0.0))

(fn HUDGetEngineRPMColor
  (return ""))

(fn HUDGetClutchStatus
  (return ""))

(fn HUDGetEngineIgnition
  (return false))