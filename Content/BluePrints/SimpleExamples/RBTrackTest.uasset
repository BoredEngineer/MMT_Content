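; Test actor for a physics-simulated tank track, with inputs for sprocket motor speed, Hook orientation and camera zoom.
; Construction places link meshes along SplineR and constrains them into a closed loop.
; Each MMT physics substep, damped spring forces hold links to a lateral plane, and GrabTracks dynamically constrains links overlapping a box to the sprocket.
; Tick rebuilds a render spline from link positions for instanced visual treads, whose spawning is switched off.
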(event EventBeginPlay)

(event Collision|EventActorBeginOverlap
  (params (OtherActor :type Actor%20Object%20Reference)))

(event EventTick
  (params (DeltaSeconds :type Float%20%28single-precision%29))
  (CallFunction|UpdateRenderingSpline)
  (bind _returnvalue (Class|PrimitiveComponent|GetPhysicsAngularVelocityinRadians (Variables|Default|GetSprocketFR) "None")))

(event EventMMTPhysicsTick
  (params (SubstepDeltaTime :type Float%20%28single-precision%29))
  (CallFunction|PullTrackwithSpring SubstepDeltaTime)
  (CallFunction|GrabTracks))

(event Input|ActionEvents|InputActionZoomIn
  (params (Key :type Key%20Structure))
  (bind _springarm (Variables|Default|GetSpringArm))
  ;[1 1 1] Camera Control
  (:Pressed
    (Variables|/Script/Engine.SpringArmComponent|SetTargetArmLength _springarm (+ (Variables|/Script/Engine.SpringArmComponent|GetTargetArmLength _springarm) -25.0))))

(event Input|ActionEvents|InputActionZoomOut
  (params (Key :type Key%20Structure))
  (bind _springarm (Variables|Default|GetSpringArm))
  ;[1 1 1] Camera Control
  (:Pressed
    (Variables|/Script/Engine.SpringArmComponent|SetTargetArmLength _springarm (+ (Variables|/Script/Engine.SpringArmComponent|GetTargetArmLength _springarm) 25.0))))

(event Input|AxisEvents|InputAxisVehicleForwardBackward
  (params (AxisValue :type Float%20%28single-precision%29))
  (Math|Float|CompareFloat AxisValue 0.0
    (:>
      _)
    (:<
      _))
  (bind _output_get (Variables|Default|SetRotationSpeedTarget (+ (Variables|Default|GetRotationSpeedTarget) (* AxisValue 0.05))))
  (Class|PhysicsConstraintComponent|SetAngularVelocityTarget (Variables|Default|GetSprocketMotor) (Math|Vector|MakeVector 0.0 _output_get 0.0)))

(event Input|AxisEvents|InputAxisVehicleRightLeft
  (params (AxisValue :type Float%20%28single-precision%29))
  (Math|Float|CompareFloat AxisValue 0.0
    (:>
      _)
    (:<
      _))
  (bind _output_get (Variables|Default|SetAngularTarget (+ (Variables|Default|GetAngularTarget) AxisValue)))
  (Class|PhysicsConstraintComponent|SetAngularOrientationTarget (Variables|Default|GetHook) (Math|Rotator|MakeRotator _output_get 0.0 0.0)))

(fn ConstructionScript
  (CallFunction|SpawnTreadsR false)
  (CallFunction|AddLinktoLinkConstraints false))

(fn SpawnTreadsR
  (params (SpawnVisual? :type Boolean))
  (bind _treadsonrightsidephysics (Variables|Default|GetTreadsOnRightSidePhysics))
  (bind _spliner (Variables|Default|GetSplineR))
  (Spline|ClearSplinePoints (Variables|Default|GetSplineForRendering) true)
  (for _index (range 0 (- _treadsonrightsidephysics 1))
    (LocalVariables|Setidx _index)
    (bind _returnvalue (AddComponent|AddStaticMeshComponent false (Math|Transform|MakeTransform (Spline|GetLocationatDistanceAlongSpline _spliner (* _index (/ (Spline|GetSplineLength _spliner) (Math|Conversions|ToFloat(Integer) _treadsonrightsidephysics))) "Local") (Math|Rotator|MakeRotator (Math|Float|SelectFloat 1.8e+02 (.roll (Spline|GetRotationatDistanceAlongSpline _spliner (* _index (/ (Spline|GetSplineLength _spliner) (Math|Conversions|ToFloat(Integer) _treadsonrightsidephysics))) "Local")) (< (.y (Class|SplineComponent|GetRightVectoratDistanceAlongSpline _spliner (* _index (/ (Spline|GetSplineLength _spliner) (Math|Conversions|ToFloat(Integer) _treadsonrightsidephysics))) "Local")) 0.0)) (.pitch (Spline|GetRotationatDistanceAlongSpline _spliner (* _index (/ (Spline|GetSplineLength _spliner) (Math|Conversions|ToFloat(Integer) _treadsonrightsidephysics))) "Local")) (.yaw (Spline|GetRotationatDistanceAlongSpline _spliner (* _index (/ (Spline|GetSplineLength _spliner) (Math|Conversions|ToFloat(Integer) _treadsonrightsidephysics))) "Local"))) "1,1,1")))
    (Utilities|Array|Add (Variables|Default|GetTreadsMeshComponentsRightSide) _returnvalue)
    (Spline|AddSplinePoint (Variables|Default|GetSplineForRendering) (Spline|GetLocationatDistanceAlongSpline _spliner (* _index (/ (Spline|GetSplineLength _spliner) (Math|Conversions|ToFloat(Integer) _treadsonrightsidephysics))) "Local") "Local" (select (== (LocalVariables|Getidx) (- (Variables|Default|GetTreadsOnRightSidePhysics) 1)) true false))
    (Utilities|Array|Add (Variables|Default|GetSprocketGrabConstraint) 0)
    (Utilities|Array|Add (Variables|Default|GetSprocketPullConstraint) 0)
    (Utilities|Array|Add (Variables|Default|GetTrackPullSpringLength) 0.0))
  (if SpawnVisual?
    (for _index_2 (range 0 (- (Variables|Default|GetTreadsOnRightSideVisual) 1))
      (Components|InstancedStaticMesh|AddInstance (Variables|Default|GetTrackSecondaryISMLeft) (Math|Transform|MakeTransform "0, 0, 0")))))

(fn UpdateRenderingSpline
  (bind _splineforrendering (Variables|Default|GetSplineForRendering))
  (bind _treadsonrightsidevisual (Variables|Default|GetTreadsOnRightSideVisual))
  (for (_array_element _array_index) (Variables|Default|GetTreadsMeshComponentsRightSide)
    (LocalVariables|Setidx _array_index)
    (Spline|SetLocationatSplinePoint (Variables|Default|GetSplineForRendering) (LocalVariables|Getidx) (Transformation|GetWorldLocation _array_element) "World" (select (== (LocalVariables|Getidx) (Utilities|Array|LastIndex (Variables|Default|GetTreadsMeshComponentsRightSide))) true false)))
  (for _index (range 0 (- _treadsonrightsidevisual 1))
    (LocalVariables|Setidx _index)
    (Components|InstancedStaticMesh|UpdateInstanceTransform (Variables|Default|GetTrackSecondaryISMLeft) (LocalVariables|Getidx) (Math|Transform|MakeTransform (Spline|GetLocationatDistanceAlongSpline _splineforrendering (* _index (/ (Spline|GetSplineLength _splineforrendering) (Math|Conversions|ToFloat(Integer) _treadsonrightsidevisual))) "Local") (Math|Rotator|MakeRotator (Math|Float|SelectFloat 1.8e+02 (.roll (Spline|GetRotationatDistanceAlongSpline _splineforrendering (* _index (/ (Spline|GetSplineLength _splineforrendering) (Math|Conversions|ToFloat(Integer) _treadsonrightsidevisual))) "Local")) (< (.y (Class|SplineComponent|GetRightVectoratDistanceAlongSpline _splineforrendering (* _index (/ (Spline|GetSplineLength _splineforrendering) (Math|Conversions|ToFloat(Integer) _treadsonrightsidevisual))) "Local")) 0.0)) (.pitch (Spline|GetRotationatDistanceAlongSpline _splineforrendering (* _index (/ (Spline|GetSplineLength _splineforrendering) (Math|Conversions|ToFloat(Integer) _treadsonrightsidevisual))) "Local")) (.yaw (Spline|GetRotationatDistanceAlongSpline _splineforrendering (* _index (/ (Spline|GetSplineLength _splineforrendering) (Math|Conversions|ToFloat(Integer) _treadsonrightsidevisual))) "Local")))) false (== (LocalVariables|Getidx) (- (Variables|Default|GetTreadsOnRightSideVisual) 1)) false)))

(fn AddLinktoLinkConstraints
  (params (OneOverOne? :type Boolean))
  (for _index (range 0 (Utilities|Array|LastIndex (Variables|Default|GetTreadsMeshComponentsRightSide)))
    (LocalVariables|SetIdx _index)
    (bind _returnvalue (AddComponent|AddPhysicsConstraintComponent true))
    (Transformation|AttachComponentToComponent _returnvalue (Utilities|Array|Get(acopy) (Variables|Default|GetTreadsMeshComponentsRightSide) (LocalVariables|GetIdx)) "None" "SnapToTarget" "SnapToTarget" "SnapToTarget" true)
    (Class|PhysicsConstraintComponent|SetDisableCollision _returnvalue (not OneOverOne?))
    (Class|PhysicsConstraintComponent|SetConstrainedComponents _returnvalue (Utilities|Array|Get(acopy) (Variables|Default|GetTreadsMeshComponentsRightSide) (select (== (LocalVariables|GetIdx) (Utilities|Array|LastIndex (Variables|Default|GetTreadsMeshComponentsRightSide))) 0 (+ (LocalVariables|GetIdx) 1))) "None" (Utilities|Array|Get(acopy) (Variables|Default|GetTreadsMeshComponentsRightSide) (LocalVariables|GetIdx)) "None")
    (Utilities|Array|Add (Variables|Default|GetLinkToLinkConstraint) _returnvalue)))

(fn GrabTracks
  (Utilities|Array|Resize (LocalVariables|GetTracksToGrab) (Utilities|Array|Length (Variables|Default|GetTreadsMeshComponentsRightSide)))
  (for _array_element (Class|PrimitiveComponent|GetOverlappingComponents (Variables|Default|GetTrackGrabBox))
    (bind (_array_element_2 _array_index) (Utilities|Array|ForEachLoopwithBreak (Variables|Default|GetTreadsMeshComponentsRightSide) :!label _label)
      (:LoopBody
        (if (== _array_element _array_element_2)
          (Utilities|Array|SetArrayElem (LocalVariables|GetTracksToGrab) _array_index true)
          (goto _label Break)))))
  (for (_array_element_3 _array_index_2) (Variables|Default|GetSprocketGrabConstraint)
    (LocalVariables|Setidx _array_index_2)
    (if (Utilities|Array|Get(acopy) (LocalVariables|GetTracksToGrab) (LocalVariables|Getidx))
      (Utilities|IsValid _array_element_3
        (:Is%20Not%20Valid
          (bind _returnvalue (AddComponent|AddPhysicsConstraintComponent true))
          (Transformation|AttachComponentToComponent _returnvalue (Utilities|Array|Get(acopy) (Variables|Default|GetTreadsMeshComponentsRightSide) (LocalVariables|Getidx)) "None" "SnapToTarget" "SnapToTarget" "SnapToTarget" false)
          (Class|PhysicsConstraintComponent|SetConstrainedComponents _returnvalue (Variables|Default|GetSprocketFR) "None" (Utilities|Array|Get(acopy) (Variables|Default|GetTreadsMeshComponentsRightSide) (LocalVariables|Getidx)) "None")
          (Utilities|Array|SetArrayElem (Variables|Default|GetSprocketGrabConstraint) (LocalVariables|Getidx) _returnvalue)
          (Rendering|Material|SetMaterial (Utilities|Array|Get(acopy) (Variables|Default|GetTreadsMeshComponentsRightSide) (LocalVariables|Getidx)) 0 "/Game/Materials/Red.Red")))
      (else
        (Utilities|IsValid _array_element_3
          (:Is%20Valid
            (Class|PhysicsConstraintComponent|BreakConstraint _array_element_3)
            (Utilities|Array|SetArrayElem (Variables|Default|GetSprocketGrabConstraint) (LocalVariables|Getidx) 0)
            (Rendering|Material|SetMaterial (Utilities|Array|Get(acopy) (Variables|Default|GetTreadsMeshComponentsRightSide) (LocalVariables|Getidx)) 0 (select (== (.Remainder (Math|Float|Division(WholeandRemainder) (Math|Conversions|ToFloat(Integer) (LocalVariables|Getidx)) 2.0)) 0.0) "/Game/Materials/Blue.Blue" "/Game/Materials/Brown.Brown"))))))))

(fn AddPullConstraint
  (for _index (range 0 (Utilities|Array|LastIndex (Variables|Default|GetTreadsMeshComponentsRightSide)))
    (LocalVariables|SetIdx _index)
    (bind _returnvalue (AddComponent|AddPhysicsConstraintComponent false (Math|Transform|MakeTransform (Math|Vector|MakeVector 0.0 101.0 0.0) "0, 0, 0" "1,1,1")))
    (Class|PhysicsConstraintComponent|SetConstrainedComponents _returnvalue (Variables|Default|GetRoot) "None" (Utilities|Array|Get(acopy) (Variables|Default|GetTreadsMeshComponentsRightSide) (LocalVariables|GetIdx)) "None")
    (Utilities|Array|Add (Variables|Default|GetSprocketPullConstraint) _returnvalue)))

(fn AdjustPullConstraint
  (for (_array_element _array_index) (Variables|Default|GetSprocketPullConstraint)
    (LocalVariables|Setidx _array_index)
    (Class|PhysicsConstraintComponent|SetLinearPositionTarget _array_element (Math|Vector|MakeVector 0.0 (- (.y (Math|Transform|InverseTransformLocation (Transformation|GetActorTransform) (Transformation|GetWorldLocation (Utilities|Array|Get(acopy) (Variables|Default|GetTreadsMeshComponentsRightSide) (LocalVariables|Getidx))))) 101.0) 0.0))
    (Development|PrintString (Utilities|String|ToString(Float) (- (.y (Math|Transform|InverseTransformLocation (Transformation|GetActorTransform) (Transformation|GetWorldLocation (Utilities|Array|Get(acopy) (Variables|Default|GetTreadsMeshComponentsRightSide) (LocalVariables|Getidx))))) 101.0)))))

(fn PullTrackwithSpring
  (params (DeltaTime :type Float%20%28single-precision%29))
  (bind _returnvalue (Class|MMTBPFunctionLibrary|MMTGetTransformComponent (Variables|Default|GetRoot) "None"))
  (LocalVariables|SetRootTransform _returnvalue)
  (for (_array_element _array_index) (Variables|Default|GetTreadsMeshComponentsRightSide)
    (LocalVariables|SetIdx _array_index)
    (bind _returnvalue_2 (Class|MMTBPFunctionLibrary|MMTGetTransformComponent _array_element "None"))
    (LocalVariables|SetSpringDirection (Math|Vector|Normalize (- (.location _returnvalue_2) (Math|Transform|TransformLocation (LocalVariables|GetRootTransform) (Math|Vector|MakeVector (.x (Math|Transform|InverseTransformLocation (LocalVariables|GetRootTransform) (.location _returnvalue_2))) 101.0 (.z (Math|Transform|InverseTransformLocation (LocalVariables|GetRootTransform) (.location _returnvalue_2))))))))
    (LocalVariables|SetNew%20SpringLength (Math|Vector|VectorLength (- (.location _returnvalue_2) (Math|Transform|TransformLocation (LocalVariables|GetRootTransform) (Math|Vector|MakeVector (.x (Math|Transform|InverseTransformLocation (LocalVariables|GetRootTransform) (.location _returnvalue_2))) 101.0 (.z (Math|Transform|InverseTransformLocation (LocalVariables|GetRootTransform) (.location _returnvalue_2))))))))
    (Class|MMTBPFunctionLibrary|MMTAddForceComponent _array_element (* (LocalVariables|GetSpringDirection) (* (+ (* 5e+02 (LocalVariables|GetNew%20SpringLength)) (|(A*(B-C)) 5e+01 0.0 (/ (- (Utilities|Array|Get(acopy) (Variables|Default|GetTrackPullSpringLength) (LocalVariables|GetIdx)) (LocalVariables|GetNew%20SpringLength)) DeltaTime))) -1.0)) true)
    (Utilities|Array|SetArrayElem (Variables|Default|GetTrackPullSpringLength) (LocalVariables|GetIdx) (LocalVariables|GetNew%20SpringLength))))

(fn SetRefPoseforConstraints
  (for (_array_element _array_index) (Variables|Default|GetLinkToLinkConstraint)
    (LocalVariables|SetIdx _array_index)
    (Class|PhysicsConstraintComponent|SetConstraintReferenceFrame _array_element "Frame1" (Math|Transform|MakeTransform (Math|Vector|MakeVector (* (LocalVariables|GetIdx) (/ (Spline|GetSplineLength (Variables|Default|GetSplineR)) (Math|Conversions|ToFloat(Integer) (Variables|Default|GetTreadsOnRightSidePhysics)))) 0.0 0.0)))))