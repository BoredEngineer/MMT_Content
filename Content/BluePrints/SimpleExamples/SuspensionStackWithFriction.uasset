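; Example four-wheeled drivable vehicle built on MMT components, with throttle, brake, Shift-held reverse, front-wheel steering, camera zoom and debug toggles.
; Each physics substep feeds engine torque to four wheel processors, updates suspension stacks and passes their contact data to friction components.
; Friction uses wheel surface velocity and active contact count, returning reaction forces to the processors.
; After physics, wheel meshes follow suspension hubs and spin from processor angular velocity.
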(event EventBeginPlay)

(event Collision|EventActorBeginOverlap
  (params (OtherActor :type Actor%20Object%20Reference)))

(event EventTick
  (params (DeltaSeconds :type Float%20%28single-precision%29))
  (CallFunction|SteerWheels DeltaSeconds))

(event EventPossessed
  (params (NewController :type Controller%20Object%20Reference))
  (Rendering|ToggleVisibility (Variables|Default|GetHelpSign) false))

(event EventUnpossessed
  (params (OldController :type Controller%20Object%20Reference))
  (Rendering|ToggleVisibility (Variables|Default|GetHelpSign) false))

(event EventMMTPhysicsTick
  (params (SubstepDeltaTime :type Float%20%28single-precision%29))
  (bind _enginetorque (Default|GetEngineTorque (Variables|Default|GetCombustionEngine)))
  (Default|SetDriveTrainTorque (Variables|Default|GetBackLeftProcessor) (Math|Float|SelectFloat (* (* _enginetorque 6.5) -1.0) (* _enginetorque 6.5) (Variables|Internal|GetReverse)))
  (Default|PhysicsUpdate (Variables|Default|GetFrontLeftProcessor) SubstepDeltaTime)
  (Class|MMTSuspensionStack|PhysicsUpdate (Variables|/Script/MMT.MMTSuspensionStackComponent|GetSuspensionStack (Variables|Default|GetFrontRightSuspensionStack)) SubstepDeltaTime)
  (CallFunction|PassCollisiontoFriction (Variables|Default|GetFrontLeftFriction) (Variables|Default|GetFrontLeftSuspensionStack))
  (CallFunction|PassCollisiontoFriction (Variables|Default|GetFrontRightFriction) (Variables|Default|GetFrontRightSuspensionStack))
  (CallFunction|PassCollisiontoFriction (Variables|Default|GetBackLeftFriction) (Variables|Default|GetBackLeftSuspensionStack))
  (CallFunction|PassCollisiontoFriction (Variables|Default|GetBackRightFriction) (Variables|Default|GetBackRightSuspensionStack))
  (CallFunction|UpdateFriction SubstepDeltaTime))

(event EventMMTAfterPhysicsTick
  (params (DeltaTime :type Float%20%28single-precision%29))
  (CallFunction|UpdateWheelPosition)
  (CallFunction|UpdateWheelAnimation (Variables|Default|GetFrontLeftWheel) (Variables|Default|GetFrontLeftProcessor) DeltaTime)
  (CallFunction|UpdateWheelAnimation (Variables|Default|GetFrontRightWheel) (Variables|Default|GetFrontRighProcessor) DeltaTime)
  (CallFunction|UpdateWheelAnimation (Variables|Default|GetBackLeftWheel) (Variables|Default|GetBackLeftProcessor) DeltaTime)
  (CallFunction|UpdateWheelAnimation (Variables|Default|GetBackRightWheel) (Variables|Default|GetBackRightProcessor) DeltaTime))

(event Input|ActionEvents|InputActionDebugMode
  (params (Key :type Key%20Structure :default "AnyKey"))
  (:Pressed
    (for _array_element (Variables|Internal|GetFrictionComponents)
      (Class|MMTFrictionComponent|ToggleDebugMode _array_element))
    (Class|MMTSuspensionStack|ToggleDebugMode (Variables|/Script/MMT.MMTSuspensionStackComponent|GetSuspensionStack (Variables|Default|GetFrontLeftSuspensionStack)))))

(event Input|ActionEvents|InputActionZoomIn
  (params (Key :type Key%20Structure :default "AnyKey"))
  (bind _springarm (Variables|Default|GetSpringArm))
  ;[1 1 1] Camera Control
  (:Pressed
    (Variables|/Script/Engine.SpringArmComponent|SetTargetArmLength _springarm (+ (Variables|/Script/Engine.SpringArmComponent|GetTargetArmLength _springarm) -25.0))))

(event Input|ActionEvents|InputActionZoomOut
  (params (Key :type Key%20Structure :default "AnyKey"))
  (bind _springarm (Variables|Default|GetSpringArm))
  ;[1 1 1] Camera Control
  (:Pressed
    (Variables|/Script/Engine.SpringArmComponent|SetTargetArmLength _springarm (+ (Variables|/Script/Engine.SpringArmComponent|GetTargetArmLength _springarm) 25.0))))

(event Input|AxisEvents|InputAxisVehicleForwardBackward
  (params (AxisValue :type Float%20%28single-precision%29))
  ;[1 1 1] Steering and Throttle input
  (Math|Float|CompareFloat AxisValue 0.0
    (:>
      (Default|SetThrottle (Variables|Default|GetCombustionEngine) AxisValue :!label _label)
      (Default|SetBrakeRatio (Variables|Default|GetFrontLeftProcessor) 0.0))
    (:==
      (goto _label))
    (:<
      (Default|SetBrakeRatio (Variables|Default|GetFrontLeftProcessor) AxisValue))))

(event Input|AxisEvents|InputAxisVehicleRightLeft
  (params (AxisValue :type Float%20%28single-precision%29))
  ;[1 1 1] Steering and Throttle input
  (Variables|Internal|SetSteerRatio AxisValue))

(event Input|KeyboardEvents|LeftShift
  (params (Key :type Key%20Structure :default "AnyKey"))
  ;[1 1 1] Steering and Throttle input
  (:Pressed
    (Variables|Internal|SetReverse true))
  (:Released
    (Variables|Internal|SetReverse false)))

(fn ConstructionScript
  (Variables|Internal|SetFrictionComponents (Utilities|Array|MakeArray (Variables|Default|GetFrontLeftFriction) (Variables|Default|GetFrontRightFriction) (Variables|Default|GetBackLeftFriction) (Variables|Default|GetBackRightFriction))))

(fn PushinRandomDirection
  (bind _returnvalue (Class|KismetMathLibrary|RandomUnitVectorinCone "0, 0,-1.000000" 0.523599))
  (bind _returnvalue_2 (Math|Random|RandomFloatinRange 3e+02 6e+02))
  (bind _chassis (Variables|Default|GetChassis))
  (bind _returnvalue_3 (* _returnvalue _returnvalue_2))
  (bind _returnvalue_4 (Transformation|GetWorldLocation _chassis))
  (Physics|AddImpulse _chassis _returnvalue_3 "None" true)
  (Rendering|Debug|DrawDebugLine _returnvalue_4 (+ _returnvalue_4 _returnvalue_3) "(R=0.895000,G=0.229743,B=0.698457,A=1.000000)" 0.25 2.0))

(fn UpdateWheelPosition
  (bind _returnvalue (Class|MMTSuspensionStack|GetWheelHubPosition (Variables|/Script/MMT.MMTSuspensionStackComponent|GetSuspensionStack (Variables|Default|GetFrontLeftSuspensionStack)) true))
  (Transformation|SetWorldLocation (Variables|Default|GetFrontLeftWheel) _returnvalue false true)
  (bind _returnvalue_2 (Class|MMTSuspensionStack|GetWheelHubPosition (Variables|/Script/MMT.MMTSuspensionStackComponent|GetSuspensionStack (Variables|Default|GetFrontRightSuspensionStack)) true))
  (Transformation|SetWorldLocation (Variables|Default|GetFrontRightWheel) _returnvalue_2 false true)
  (bind _returnvalue_3 (Class|MMTSuspensionStack|GetWheelHubPosition (Variables|/Script/MMT.MMTSuspensionStackComponent|GetSuspensionStack (Variables|Default|GetBackLeftSuspensionStack)) true))
  (Transformation|SetWorldLocation (Variables|Default|GetBackLeftWheel) _returnvalue_3 false true)
  (bind _returnvalue_4 (Class|MMTSuspensionStack|GetWheelHubPosition (Variables|/Script/MMT.MMTSuspensionStackComponent|GetSuspensionStack (Variables|Default|GetBackRightSuspensionStack)) true))
  (Transformation|SetWorldLocation (Variables|Default|GetBackRightWheel) _returnvalue_4 false true))

(fn PassCollisiontoFriction
  (params (FrictionComponent :type MMT%20Friction%20Component%20Object%20Reference) (SuspensionStack :type MMT%20Suspension%20Stack%20Component%20Object%20Reference))
  ;[1 1 1] When suspension stack finds location for the wheel, it records data about where wheel would collide with the ground.
  ; This collision data is passed to friction component to calculate friction force.
  (bind (_bpointactive _forceatpoint _pointlocation _surfacenormal _surfacephysicalmaterial _surfacevelocity) (Class|MMTSuspensionStack|GetContactData (Variables|/Script/MMT.MMTSuspensionStackComponent|GetSuspensionStack SuspensionStack)))
  (Class|MMTFrictionComponent|ResetFrictionPoints FrictionComponent)
  (if _bpointactive
    (Class|MMTFrictionComponent|RegisterFrictionPoint FrictionComponent _forceatpoint false _pointlocation _surfacenormal _surfacephysicalmaterial _surfacevelocity)))

(fn UpdateFriction
  (params (DeltaTime :type Float%20%28single-precision%29))
  (LocalVariables|SetDT DeltaTime)
  ;[1 1 1] First we need to count total amount of friction points that need to be processed. Friction point is counted as active if it received
  ; a valid contact point information, from another component, such as suspension stack.
  (for _array_element (Variables|Internal|GetFrictionComponents)
    (bind _returnvalue (Class|MMTFrictionComponent|IsFrictionPointActive _array_element))
    (if _returnvalue
      (Math|Integer|IncrementInt (LocalVariables|GetPointsCount))))
  (bind _linearvelocity (Default|GetTrackLinearVelocityVector (Variables|Default|GetFrontLeftProcessor)))
  (Class|MMTFrictionComponent|SetFrictionSurfaceVelocity (Variables|Default|GetFrontLeftFriction) _linearvelocity)
  (bind _linearvelocity_2 (Default|GetTrackLinearVelocityVector (Variables|Default|GetFrontRighProcessor)))
  (Class|MMTFrictionComponent|SetFrictionSurfaceVelocity (Variables|Default|GetFrontRightFriction) _linearvelocity_2)
  (bind _linearvelocity_3 (Default|GetTrackLinearVelocityVector (Variables|Default|GetBackLeftProcessor)))
  (Class|MMTFrictionComponent|SetFrictionSurfaceVelocity (Variables|Default|GetBackLeftFriction) _linearvelocity_3)
  (bind _linearvelocity_4 (Default|GetTrackLinearVelocityVector (Variables|Default|GetBackRightProcessor)))
  (Class|MMTFrictionComponent|SetFrictionSurfaceVelocity (Variables|Default|GetBackRightFriction) _linearvelocity_4)
  (bind (_normalizedreactionforce _rollingfrictionforce) (Class|MMTFrictionComponent|PhysicsUpdate (Variables|Default|GetFrontLeftFriction) (Math|Conversions|ToFloat(Integer) (LocalVariables|GetPointsCount)) (LocalVariables|GetDT)))
  (Default|SetTrackApplicationForce (Variables|Default|GetFrontLeftProcessor) _normalizedreactionforce _rollingfrictionforce)
  (bind (_normalizedreactionforce_2 _rollingfrictionforce_2) (Class|MMTFrictionComponent|PhysicsUpdate (Variables|Default|GetFrontRightFriction) (Math|Conversions|ToFloat(Integer) (LocalVariables|GetPointsCount)) (LocalVariables|GetDT)))
  (Default|SetTrackApplicationForce (Variables|Default|GetFrontRighProcessor) _normalizedreactionforce_2 _rollingfrictionforce_2)
  (bind (_normalizedreactionforce_3 _rollingfrictionforce_3) (Class|MMTFrictionComponent|PhysicsUpdate (Variables|Default|GetBackLeftFriction) (Math|Conversions|ToFloat(Integer) (LocalVariables|GetPointsCount)) (LocalVariables|GetDT)))
  (Default|SetTrackApplicationForce (Variables|Default|GetBackLeftProcessor) _normalizedreactionforce_3 _rollingfrictionforce_3)
  (bind (_normalizedreactionforce_4 _rollingfrictionforce_4) (Class|MMTFrictionComponent|PhysicsUpdate (Variables|Default|GetBackRightFriction) (Math|Conversions|ToFloat(Integer) (LocalVariables|GetPointsCount)) (LocalVariables|GetDT)))
  (Default|SetTrackApplicationForce (Variables|Default|GetBackRightProcessor) _normalizedreactionforce_4 _rollingfrictionforce_4))

(fn UpdateWheelAnimation
  (params (Wheelmesh :type Static%20Mesh%20Component%20Object%20Reference) (WheelProcessor :type Track%20Transmission%20Processor%20Object%20Reference) (DeltaTime :type Float%20%28single-precision%29))
  (bind _sprocketangularvelocity (Default|GetSprocketAngularVelocity WheelProcessor))
  (Transformation|SetRelativeRotation Wheelmesh (Math|Rotator|CombineRotators (Variables|/Script/Engine.SceneComponent|GetRelativeRotation Wheelmesh) (Math|Rotator|MakeRotator 0.0 (* (* (Math|Trig|RadiansToDegrees _sprocketangularvelocity) DeltaTime) -1.0) 0.0)) false true))

(fn SteerWheels
  (params (DeltaTime :type Float%20%28single-precision%29))
  (bind _frontrightsuspensionstack (Variables|Default|GetFrontRightSuspensionStack))
  (bind _frontleftsuspensionstack (Variables|Default|GetFrontLeftSuspensionStack))
  (bind _relativerotation (Variables|/Script/Engine.SceneComponent|GetRelativeRotation _frontleftsuspensionstack))
  (bind _relativerotation_2 (Variables|/Script/Engine.SceneComponent|GetRelativeRotation _frontrightsuspensionstack))
  (Transformation|SetRelativeRotation _frontleftsuspensionstack (Math|Rotator|MakeRotator (.roll _relativerotation) (.pitch _relativerotation) (Math|Interpolation|FInterptoConstant (.yaw _relativerotation) (* (Variables|Internal|GetSteerRatio) (Variables|Default|GetMaxSteerAngle)) DeltaTime 1e+02)) false false)
  (Transformation|SetRelativeRotation _frontrightsuspensionstack (Math|Rotator|MakeRotator (.roll _relativerotation_2) (.pitch _relativerotation_2) (Math|Interpolation|FInterptoConstant (.yaw _relativerotation_2) (* (Variables|Internal|GetSteerRatio) (Variables|Default|GetMaxSteerAngle)) DeltaTime 5e+01)) false false))