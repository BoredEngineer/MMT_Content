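; Simple MMT physics example pawn that tests static friction on a slope, with camera zoom and debug toggles.
; Each physics substep traces below the chassis, derives the slope angle and applies an uphill force cancelling gravity's slope component only within the Coulomb limit, drawing debug values.
; Chassis hits still register contacts on CenterFriction, but the component-based UpdateFriction path is disconnected, leaving this hand-computed reference friction active.
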(event OnComponentHit(Chassis)
  (params (HitComponent :type Primitive%20Component%20Object%20Reference) (OtherActor :type Actor%20Object%20Reference) (OtherComp :type Primitive%20Component%20Object%20Reference) (NormalImpulse :type Vector) (Hit :type Hit%20Result%20Structure%20%28by%20ref%29))
  (if (.bblockinghit Hit)
    (CallFunction|ResetFrictionPoints)
    (Class|MMTFrictionComponent|RegisterFrictionPoint (Variables|Default|GetCenterFriction) (* NormalImpulse -1.0) true (.impactpoint Hit) (.impactnormal Hit) (.physmat Hit) "0, 0, 0")))

(event EventBeginPlay)

(event Collision|EventActorBeginOverlap
  (params (OtherActor :type Actor%20Object%20Reference)))

(event EventTick
  (params (DeltaSeconds :type Float%20%28single-precision%29))
  (Rendering|Debug|DrawDebugString (Transformation|GetWorldLocation (Variables|Default|GetChassis)) (Utilities|String|Append "Friction magnitude: " (Utilities|String|ToString(Float) (Variables|Default|GetFrictionForceAmplitude))) 0 "(R=1.000000,G=1.000000,B=1.000000,A=1.000000)"))

(event EventPossessed
  (params (NewController :type Controller%20Object%20Reference))
  (Rendering|ToggleVisibility (Variables|Default|GetHelpSign) false))

(event EventUnpossessed
  (params (OldController :type Controller%20Object%20Reference))
  (Rendering|ToggleVisibility (Variables|Default|GetHelpSign) false))

(event EventMMTPhysicsTick
  (params (SubstepDeltaTime :type Float%20%28single-precision%29))
  (Variables|Default|SetIsResetFrictionPoints true)
  (CallFunction|ComputeandApplyReferenceFriction SubstepDeltaTime)
  (Class|PrimitiveComponent|WakeRigidBody (Variables|Default|GetChassis) "None"))

(event EventMMTAfterPhysicsTick
  (params (DeltaTime :type Float%20%28single-precision%29)))

(event Input|ActionEvents|InputActionDebugMode
  (params (Key :type Key%20Structure :default "AnyKey"))
  (:Pressed
    (Utilities|FlowControl|Sequence
      (:then_0
        (for _array_element (Variables|Internal|GetFrictionComponents)
          (Class|MMTFrictionComponent|ToggleDebugMode _array_element))))))

(event Input|ActionEvents|InputActionZoomIn
  (params (Key :type Key%20Structure :default "AnyKey"))
  (bind _springarm (Variables|Default|GetSpringArm))
  ;[1 1 1] Camera Control
  (:Pressed
    (Variables|/Script/Engine.SpringArmComponent|SetTargetArmLength _springarm (+ (Variables|/Script/Engine.SpringArmComponent|GetTargetArmLength _springarm) -25.0))))

(event Input|ActionEvents|InputActionZoomOut
  (params (Key :type Key%20Structure :default "AnyKey"))
  (bind _springarm (Variables|Default|GetSpringArm))
  ;[1 1 1] Camera Control
  (:Pressed
    (Variables|/Script/Engine.SpringArmComponent|SetTargetArmLength _springarm (+ (Variables|/Script/Engine.SpringArmComponent|GetTargetArmLength _springarm) 25.0))))

(fn ConstructionScript
  (Variables|Internal|SetFrictionComponents (Utilities|Array|MakeArray (Variables|Default|GetCenterFriction) (Variables|Default|GetFrontRightFriction) (Variables|Default|GetBackLeftFriction) (Variables|Default|GetBackRightFriction))))

(fn PushinRandomDirection
  (bind _returnvalue (Class|KismetMathLibrary|RandomUnitVectorinCone "0, 0,-1.000000" 0.523599))
  (bind _returnvalue_2 (Math|Random|RandomFloatinRange 3e+02 6e+02))
  (bind _chassis (Variables|Default|GetChassis))
  (bind _returnvalue_3 (* _returnvalue _returnvalue_2))
  (bind _returnvalue_4 (Transformation|GetWorldLocation _chassis))
  (Physics|AddImpulse _chassis _returnvalue_3 "None" true)
  (Rendering|Debug|DrawDebugLine _returnvalue_4 (+ _returnvalue_4 _returnvalue_3) "(R=0.895000,G=0.229743,B=0.698457,A=1.000000)" 0.25 2.0))

(fn UpdateFriction
  (params (DeltaTime :type Float%20%28single-precision%29))
  (LocalVariables|SetDT DeltaTime)
  ;[1 1 1] First we need to count total amount of friction points that need to be processed. Friction point is counted as active if it received
  ; a valid contact point information, from another component, such as suspension stack.
  (for _array_element (Variables|Internal|GetFrictionComponents)
    (bind _returnvalue (Class|MMTFrictionComponent|IsFrictionPointActive _array_element))
    (if _returnvalue
      (Math|Integer|IncrementInt (LocalVariables|GetPointsCount))))
  (Class|MMTFrictionComponent|PhysicsUpdate (Variables|Default|GetCenterFriction) (Math|Conversions|ToFloat(Integer) (LocalVariables|GetPointsCount)) (LocalVariables|GetDT))
  (bind _returnvalue_2 (Class|MMTFrictionComponent|GetFrictionForce (Variables|Default|GetCenterFriction)))
  (Variables|Default|SetFrictionForceAmplitude (Math|Vector|VectorLength _returnvalue_2)))

(fn ComputeandApplyReferenceFriction
  (params (DeltaTime :type Float%20%28single-precision%29))
  (bind _chassis (Variables|Default|GetChassis))
  (bind _chassis_2 (Variables|Default|GetChassis))
  (bind _chassis_3 (Variables|Default|GetChassis))
  (bind _chassis_4 (Variables|Default|GetChassis))
  (bind _returnvalue (Transformation|GetWorldLocation _chassis_2))
  (bind _returnvalue_2 (Physics|GetMass _chassis))
  (bind _returnvalue_3 (Transformation|GetWorldLocation _chassis_3))
  (bind _returnvalue_4 (* _returnvalue_2 9.8e+02))
  (LocalVariables|SetDT DeltaTime)
  (bind _outhit (Collision|LineTraceByChannel _returnvalue_3 (+ _returnvalue_3 (* (Math|Vector|GetUpVector _chassis_3) -1e+02)) "TraceTypeQuery1" false 0 "ForOneFrame"))
  (if (.bblockinghit _outhit)
    (LocalVariables|SetImpactNormal (.impactnormal _outhit))
    (LocalVariables|SetFrictionDirection (Math|Vector|Normalize (Math|Vector|ProjectVectorontoPlane "0, 0,1.000000" (.impactnormal _outhit))))
    (LocalVariables|SetCosA (Math|Vector|DotProduct (LocalVariables|GetFrictionDirection) (Math|Vector|Normalize (Math|Vector|MakeVector (.X (Math|Vector|BreakVector (LocalVariables|GetFrictionDirection))) (.Y (Math|Vector|BreakVector (LocalVariables|GetFrictionDirection))) 0.0))))
    (Rendering|Debug|DrawDebugString (+ (Transformation|GetWorldLocation _chassis_4) (* (Math|Vector|GetUpVector _chassis_4) 1e+02)) (Utilities|String|Append "Slope angle: " (Utilities|String|ToString(Float) (Class|KismetMathLibrary|DegAtan2 (Math|Vector|VectorLength (Math|Vector|CrossProduct (LocalVariables|GetFrictionDirection) (Math|Vector|Normalize (Math|Vector|MakeVector (.X (Math|Vector|BreakVector (LocalVariables|GetFrictionDirection))) (.Y (Math|Vector|BreakVector (LocalVariables|GetFrictionDirection))) 0.0)))) (Math|Vector|DotProduct (LocalVariables|GetFrictionDirection) (Math|Vector|Normalize (Math|Vector|MakeVector (.X (Math|Vector|BreakVector (LocalVariables|GetFrictionDirection))) (.Y (Math|Vector|BreakVector (LocalVariables|GetFrictionDirection))) 0.0)))))) 0 "(R=1.000000,G=1.000000,B=1.000000,A=1.000000)")
    (LocalVariables|SetSinA (Math|Trig|Sin(Degrees) (Class|KismetMathLibrary|DegAtan2 (Math|Vector|VectorLength (Math|Vector|CrossProduct (LocalVariables|GetFrictionDirection) (Math|Vector|Normalize (Math|Vector|MakeVector (.X (Math|Vector|BreakVector (LocalVariables|GetFrictionDirection))) (.Y (Math|Vector|BreakVector (LocalVariables|GetFrictionDirection))) 0.0)))) (Math|Vector|DotProduct (LocalVariables|GetFrictionDirection) (Math|Vector|Normalize (Math|Vector|MakeVector (.X (Math|Vector|BreakVector (LocalVariables|GetFrictionDirection))) (.Y (Math|Vector|BreakVector (LocalVariables|GetFrictionDirection))) 0.0))))))
    (bind _output_get (LocalVariables|SetFrictionForceAmplitudeLoc (* _returnvalue_4 (LocalVariables|GetSinA))))
    (if (and (!= _output_get 0.0) (<= _output_get (* _returnvalue_4 (* (LocalVariables|GetCosA) (Variables|Default|GetFrictionCoefficient)))))
      (Variables|Default|SetFrictionForceAmplitude (LocalVariables|GetFrictionForceAmplitudeLoc))
      (Class|MMTBPFunctionLibrary|MMTAddForceComponent (Variables|Default|GetChassis) (* (LocalVariables|GetFrictionDirection) (LocalVariables|GetFrictionForceAmplitudeLoc)) false)
      (Rendering|Debug|DrawDebugLine _returnvalue (+ _returnvalue (* (LocalVariables|GetFrictionDirection) (LocalVariables|GetFrictionForceAmplitudeLoc))) "(R=1.000000,G=0.055000,B=0.671518,A=1.000000)" 0.0 5.0))))

(fn ResetFrictionPoints
  (if (Variables|Default|GetIsResetFrictionPoints)
    (Variables|Default|SetIsResetFrictionPoints false)
    (Class|MMTFrictionComponent|ResetFrictionPoints (Variables|Internal|GetFrictionComponents))))