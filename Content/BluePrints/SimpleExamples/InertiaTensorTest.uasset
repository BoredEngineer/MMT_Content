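; Test Blueprint for inspecting and overriding the inertia tensor of a physics StaticMesh, with spring-arm zoom.
; After a short delay, Q prints the current tensor and E sets it to a unit vector through MMTSetInertiaTensor.
; A, S and D apply a large torque about the mesh's local X, Y and Z axes to show the response.
; All three torque messages say "X axis", differing only in color.
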(event EventBeginPlay)

(event Collision|EventActorBeginOverlap
  (params (OtherActor :type Actor%20Object%20Reference)))

(event EventTick
  (params (DeltaSeconds :type Float%20%28single-precision%29)))

(event Input|ActionEvents|InputActionZoomIn
  (params (Key :type Key%20Structure :default "AnyKey"))
  (bind _springarm (Variables|Default|GetSpringArm))
  (:Pressed
    (Variables|/Script/Engine.SpringArmComponent|SetTargetArmLength _springarm (+ (Variables|/Script/Engine.SpringArmComponent|GetTargetArmLength _springarm) -25.0))))

(event Input|ActionEvents|InputActionZoomOut
  (params (Key :type Key%20Structure :default "AnyKey"))
  (bind _springarm (Variables|Default|GetSpringArm))
  (:Pressed
    (Variables|/Script/Engine.SpringArmComponent|SetTargetArmLength _springarm (+ (Variables|/Script/Engine.SpringArmComponent|GetTargetArmLength _springarm) 25.0))))

(event Input|KeyboardEvents|D
  (params (Key :type Key%20Structure :default "AnyKey"))
  (:Pressed
    (Utilities|FlowControl|Delay 0.2)
    (Class|PrimitiveComponent|AddTorque (Variables|Default|GetStaticMesh) (Math|Transform|TransformDirection (Transformation|GetWorldTransform (Variables|Default|GetStaticMesh)) "0.000000,0.000000,5000000.000000") "None" false)
    (Development|PrintString "added Torque in X axis" true true "(R=0.000000,G=0.038215,B=1.000000,A=1.000000)")))

(event Input|KeyboardEvents|E
  (params (Key :type Key%20Structure :default "AnyKey"))
  (bind _returnvalue (Math|Vector|MakeVector 1.0 1.0 1.0))
  (:Pressed
    (Utilities|FlowControl|Delay 0.2)
    (Class|MMTBPFunctionLibrary|MMTSetInertiaTensor (Variables|Default|GetStaticMesh) _returnvalue)
    (Development|PrintString (Utilities|String|Append "new Inertia Tensor: " (Utilities|String|ToString(Vector) _returnvalue)) true true "(R=0.000000,G=0.809316,B=1.000000,A=1.000000)")))

(event Input|KeyboardEvents|A
  (params (Key :type Key%20Structure :default "AnyKey"))
  (:Pressed
    (Utilities|FlowControl|Delay 0.2)
    (Class|PrimitiveComponent|AddTorque (Variables|Default|GetStaticMesh) (Math|Transform|TransformDirection (Transformation|GetWorldTransform (Variables|Default|GetStaticMesh)) "5000000.000000, 0,0.000000") "None" false)
    (Development|PrintString "added Torque in X axis" true true "(R=1.000000,G=0.000000,B=0.046095,A=1.000000)")))

(event Input|KeyboardEvents|S
  (params (Key :type Key%20Structure :default "AnyKey"))
  (:Pressed
    (Utilities|FlowControl|Delay 0.2)
    (Class|PrimitiveComponent|AddTorque (Variables|Default|GetStaticMesh) (Math|Transform|TransformDirection (Transformation|GetWorldTransform (Variables|Default|GetStaticMesh)) "0.000000,5000000.000000, 0") "None" false)
    (Development|PrintString "added Torque in X axis" true true "(R=0.015103,G=1.000000,B=0.000000,A=1.000000)")))

(event Input|KeyboardEvents|Q
  (params (Key :type Key%20Structure :default "AnyKey"))
  (:Pressed
    (Utilities|FlowControl|Delay 0.2)
    (Development|PrintString (Utilities|String|Append "Inertia Tensor: " (Utilities|String|ToString(Vector) (Class|PrimitiveComponent|GetInertiaTensor (Variables|Default|GetStaticMesh) "None"))))))

(fn ConstructionScript)