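; Example drivable car pawn testing an MMT drivetrain: engine, dry clutch, drive shaft and one wheel's ground friction, with throttle, brake, clutch and starter input.
; Each physics substep passes torque engine-to-shaft and back through the clutch, sharing angular speed when locked.
; Wheel hit events feed anisotropic friction points, but the shaft receives zero reaction force.
; Steering is empty; HUD getters for gearbox and speed are stubs.
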(event OnComponentHit(CollisionWheelBR)
  (params (HitComponent :type Primitive%20Component%20Object%20Reference) (OtherActor :type Actor%20Object%20Reference) (OtherComp :type Primitive%20Component%20Object%20Reference) (NormalImpulse :type Vector) (Hit :type Hit%20Result%20Structure%20%28by%20ref%29))
  (if (.bblockinghit Hit)
    (if (Variables|Default|GetIsResetFrictionPoints)
      (Default|ResetFrictionPoints (Variables|Default|GetTrackAnisotropicFriction))
      (Variables|Default|SetIsResetFrictionPoints false))
    (Default|RegisterFrictionPoint (Variables|Default|GetTrackAnisotropicFriction) "0, 0, 0" (* NormalImpulse -1.0) (.impactpoint Hit) (.impactnormal Hit))))

(event EventBeginPlay)

(event Collision|EventActorBeginOverlap
  (params (OtherActor :type Actor%20Object%20Reference)))

(event EventMMTPhysicsTick
  (params (SubstepDeltaTime :type Float%20%28single-precision%29))
  (Default|PhysicsUpdate (Variables|Default|GetCombustionEngineAdvanced) SubstepDeltaTime)
  (CallFunction|UpdateTorquefromEnginetoShaft SubstepDeltaTime)
  (Default|PhysicsUpdate (Variables|Default|GetDriveShaft) SubstepDeltaTime)
  (CallFunction|UpdateGroundFriction SubstepDeltaTime)
  (CallFunction|UpdateTorquefromShafttoEngine SubstepDeltaTime))

(event EventTick
  (params (DeltaSeconds :type Float%20%28single-precision%29))
  (Variables|Default|SetIsResetFrictionPoints true)
  (Class|PrimitiveComponent|WakeAllRigidBodies (Variables|Default|GetChassis))
  (Default|AnimateEngine (Variables|Default|GetCombustionEngineAdvanced) DeltaSeconds)
  (Default|AnimateShaft (Variables|Default|GetDriveShaft) DeltaSeconds)
  (CallFunction|AnimateClutch)
  (bind _angularspeed (Default|GetAngularSpeed (Variables|Default|GetCombustionEngineAdvanced)))
  (Rendering|Debug|DrawDebugString (Transformation|GetWorldLocation (Variables|Default|GetCrankShaft)) (Utilities|String|ToString(Float) _angularspeed) 0 "(R=1.000000,G=1.000000,B=1.000000,A=1.000000)")
  (Rendering|Debug|DrawDebugString (Transformation|GetWorldLocation (Variables|Default|GetAxle)) (Utilities|String|ToString(Float) (Variables|/Game/BluePrints/ReUsableComponents/DriveComponents/DriveShaft.DriveShaft_C|GetAngularSpeed (Variables|Default|GetDriveShaft))) 0 "(R=1.000000,G=1.000000,B=1.000000,A=1.000000)")
  (bind _clutchstatus (Default|GetClutchStatus (Variables|Default|GetDryClutch)))
  (Rendering|Debug|DrawDebugString (Transformation|GetWorldLocation (Variables|Default|GetDryClutch)) _clutchstatus 0 "(R=1.000000,G=1.000000,B=1.000000,A=1.000000)"))

(event EventPossessed
  (params (NewController :type Controller%20Object%20Reference))
  ;[1 1 1] Add and remove vehicle HUD
  (bind _asmmtcontroller (Utilities|Casting|CastToMMTController NewController))
  (Default|CreateMachineryWidget _asmmtcontroller (Variables|Default|GetHUDWidgetClass))
  (Rendering|ToggleVisibility (Variables|Default|GetHelpSign) false))

(event EventUnpossessed
  (params (OldController :type Controller%20Object%20Reference))
  ;[1 1 1] Add and remove vehicle HUD
  (bind _asmmtcontroller (Utilities|Casting|CastToMMTController OldController))
  (Default|RemoveMachineryWidget _asmmtcontroller)
  (Rendering|ToggleVisibility (Variables|Default|GetHelpSign) false))

(event Input|ActionEvents|InputActionDebugMode
  (params (Key :type Key%20Structure :default "AnyKey"))
  (:Pressed
    (Default|ToggleDebugOn/off (Variables|Default|GetPSSVisualDebugger))))

(event Input|ActionEvents|InputActionZoomIn
  (params (Key :type Key%20Structure :default "AnyKey"))
  (bind _springarm (Variables|Default|GetSpringArm))
  ;[1 1 1] Camera Control
  (:Pressed
    (Variables|/Script/Engine.SpringArmComponent|SetTargetArmLength _springarm (+ (Variables|/Script/Engine.SpringArmComponent|GetTargetArmLength _springarm) -25.0))))

(event Input|ActionEvents|InputActionZoomOut
  (params (Key :type Key%20Structure :default "AnyKey"))
  (bind _springarm (Variables|Default|GetSpringArm))
  ;[1 1 1] Camera Control
  (:Pressed
    (Variables|/Script/Engine.SpringArmComponent|SetTargetArmLength _springarm (+ (Variables|/Script/Engine.SpringArmComponent|GetTargetArmLength _springarm) 25.0))))

(event Input|AxisEvents|InputAxisVehicleForwardBackward
  (params (AxisValue :type Float%20%28single-precision%29))
  ;[1 1 1] Steering and throttle controls
  (Math|Float|CompareFloat AxisValue 0.0
    (:>
      (Default|SetThrottle (Variables|Default|GetCombustionEngineAdvanced) AxisValue :!label _label)
      (Default|SetBrakeRatio (Variables|Default|GetDriveShaft) 0.0))
    (:==
      (goto _label))
    (:<
      (Default|SetBrakeRatio (Variables|Default|GetDriveShaft) 1.0))))

(event Input|AxisEvents|InputAxisVehicleRightLeft
  (params (AxisValue :type Float%20%28single-precision%29))
  ;[1 1 1] Steering and throttle controls
  (Math|Float|CompareFloat AxisValue 0.0))

(event Input|KeyboardEvents|LeftShift
  (params (Key :type Key%20Structure :default "AnyKey"))
  ;[1 1 1] Steering and throttle controls
  (:Pressed
    (Default|PressClutch (Variables|Default|GetDryClutch) 0.0))
  (:Released
    (Default|PressClutch (Variables|Default|GetDryClutch) 1.0)))

(event Input|KeyboardEvents|E
  (params (Key :type Key%20Structure :default "AnyKey"))
  (bind _combustionengineadvanced (Variables|Default|GetCombustionEngineAdvanced))
  ;[1 1 1] Steering and throttle controls
  (:Pressed
    (Default|SetStarter _combustionengineadvanced true))
  (:Released
    (Default|SetStarter _combustionengineadvanced false)))

(fn ConstructionScript
  (Rendering|Components|TextRender|SetText (Variables|Default|GetHelpSign) (Utilities|Text|MakeLiteralText "Press 3 to posses")))

(fn UpdateTorquefromEnginetoShaft
  (params (DeltaTime :type Float%20%28single-precision%29))
  (bind _driveshaft (Variables|Default|GetDriveShaft))
  (bind (_torque _angularspeed _momentofinertia _dampingrate) (Default|GetDataforTorqueTransfer (Variables|Default|GetCombustionEngineAdvanced)))
  (Rendering|Debug|DrawDebugString (+ (Transformation|GetWorldLocation (Variables|Default|GetCrankShaft)) "0, 0,100.000000") (Utilities|String|Append "Torque IN: " (Utilities|String|ToString(Float) _torque)) 0 "(R=1.000000,G=1.000000,B=1.000000,A=1.000000)")
  (bind (_torque_2 _angularspeed_2 _momentofinertia_2 _dampingrate_2) (Default|GetDataforTorqueTransfer (Variables|Default|GetDriveShaft)))
  (bind (_torqueout _isclutchlocked) (Default|CalculateTorqueTransfer (Variables|Default|GetDryClutch) _torque _angularspeed _angularspeed_2 _momentofinertia _momentofinertia_2 _dampingrate _dampingrate_2))
  (Rendering|Debug|DrawDebugString (+ (Transformation|GetWorldLocation (Variables|Default|GetAxle)) "0, 0,100.000000") (Utilities|String|Append "Torque OUT: " (Utilities|String|ToString(Float) _torqueout)) 0 "(R=1.000000,G=1.000000,B=1.000000,A=1.000000)")
  (if _isclutchlocked
    (Default|SetLockedAngularSpeedandTorque _driveshaft _angularspeed _torqueout)
    (else
      (Default|UpdateAngularSpeedfromTorque _driveshaft _torqueout DeltaTime))))

(fn UpdateTorquefromShafttoEngine
  (params (DeltaTime :type Float%20%28single-precision%29))
  (bind _combustionengineadvanced (Variables|Default|GetCombustionEngineAdvanced))
  (bind (_torque _angularspeed _momentofinertia _dampingrate) (Default|GetDataforTorqueTransfer (Variables|Default|GetDriveShaft)))
  (Rendering|Debug|DrawDebugString (+ (Transformation|GetWorldLocation (Variables|Default|GetAxle)) "0, 0,75.000000") (Utilities|String|Append "Torque IN: " (Utilities|String|ToString(Float) _torque)) 0 "(R=1.000000,G=1.000000,B=1.000000,A=1.000000)")
  (bind (_torque_2 _angularspeed_2 _momentofinertia_2 _dampingrate_2) (Default|GetDataforTorqueTransfer (Variables|Default|GetCombustionEngineAdvanced)))
  (bind (_torqueout _isclutchlocked) (Default|CalculateTorqueTransfer (Variables|Default|GetDryClutch) _torque _angularspeed _angularspeed_2 _momentofinertia _momentofinertia_2 _dampingrate _dampingrate_2))
  (Rendering|Debug|DrawDebugString (+ (Transformation|GetWorldLocation (Variables|Default|GetCrankShaft)) "0, 0,75.000000") (Utilities|String|Append "Torque OUT: " (Utilities|String|ToString(Float) _torqueout)) 0 "(R=1.000000,G=1.000000,B=1.000000,A=1.000000)")
  (if _isclutchlocked
    (Default|SetLockedAngularSpeedandTorque _combustionengineadvanced _angularspeed _torqueout)
    (else
      (Default|UpdateAngularSpeedfromTorque _combustionengineadvanced _torqueout DeltaTime))))

(fn AnimateClutch
  (bind _clutchplateposition (Default|GetClutchStatus (Variables|Default|GetDryClutch)))
  (Transformation|SetRelativeLocation (Variables|Default|GetClutchDiskE) (Math|Vector|MakeVector (* (- 1.0 _clutchplateposition) -5.0) 0.0 0.0) false false))

(fn UpdateGroundFriction
  (params (DeltaTIme :type Float%20%28single-precision%29))
  (Default|UpdateTrackData (Variables|Default|GetTrackAnisotropicFriction) (* (Math|Transform|TransformDirection (Transformation|GetWorldTransform (Variables|Default|GetCollisionWheelBR)) "1.000000, 0, 0") (* (Variables|/Game/BluePrints/ReUsableComponents/DriveComponents/DriveShaft.DriveShaft_C|GetAngularSpeed (Variables|Default|GetDriveShaft)) 2e+01 1.0)))
  (Default|PhysicsUpdate (Variables|Default|GetTrackAnisotropicFriction) 1 DeltaTIme)
  (Default|ProcessReactionForce (Variables|Default|GetDriveShaft) "0, 0, 0" DeltaTIme))

(fn AddDebugCoordinateSystem
  (params (DebugCoordinateSystem :type Debug%20Coordinate%20System%20Structure))
  (Default|AddDebugCoordinateSystem (Variables|Default|GetPSSVisualDebugger) DebugCoordinateSystem)
  (return false))

(fn AddDebugFloatGraph
  (params (DebugFloatGraph :type Debug%20Float%20Graph%20Input%20Structure))
  (Default|AddDebugFloatGraph (Variables|Default|GetPSSVisualDebugger) DebugFloatGraph)
  (return false))

(fn AddDebugLine
  (params (DebugLine :type Debug%20Line%20Structure))
  (Default|AddDebugLine (Variables|Default|GetPSSVisualDebugger) DebugLine)
  (return false))

(fn AddDebugString
  (params (DebugString :type Debug%20String%20Structure))
  (Default|AddDebugString (Variables|Default|GetPSSVisualDebugger) DebugString)
  (return false))

(fn HUDGetClutchStatus
  (bind _clutchstatus (Default|GetClutchStatus (Variables|Default|GetDryClutch)))
  (return _clutchstatus))

(fn HUDGetEngineIgnition
  (return (Variables|/Game/Blueprints/ReUsableComponents/Engines/CombustionEngineAdvanced.CombustionEngineAdvanced_C|GetIsIgnitionON (Variables|Default|GetCombustionEngineAdvanced))))

(fn HUDGetEngineRPM
  (bind _enginerpm (Default|GetEngineRPMGUI (Variables|Default|GetCombustionEngineAdvanced)))
  (return _enginerpm))

(fn HUDGetEngineRPMColor
  (bind _color (Default|GetEngineRPMColor (Variables|Default|GetCombustionEngineAdvanced)))
  (return _color))

(fn HUDGetEngineStarter
  (return false))

(fn HUDGetEngineTorque
  (bind _enginetorque (Default|GetEngineTorque (Variables|Default|GetCombustionEngineAdvanced)))
  (return _enginetorque))

(fn HUDGetGearBoxInfo
  (return 0 0 false))

(fn HUDGetThrottle
  (bind _enginethrottle (Default|GetThrottle (Variables|Default|GetCombustionEngineAdvanced)))
  (return _enginethrottle))

(fn HUDGetVehicleSpeed
  (return 0.0))