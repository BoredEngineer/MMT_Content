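; Simple example actor that uses MMT substepped physics to keep its body upright along a configurable world direction.
; Each physics substep reads the Top and Bottom socket transforms and applies force at Top toward a target point offset from Bottom.
; Force scales with axis alignment, damped by the change rate of distance to target.
; A separate function applies a random impulse with a debug line.
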(event EventBeginPlay)

(event EventActorBeginOverlap
  (params (OtherActor :type Actor%20Object%20Reference)))

(event EventTick
  (params (DeltaSeconds :type Float%20%28single-precision%29)))

(event EventMMTPhysicsTick
  (params (SubstepDeltaTime :type Float%20%28single-precision%29))
  (CallFunction|ApplyUpRightCorrection SubstepDeltaTime))

(fn ConstructionScript
  (Variables|Default|SetDesiredWorldDirectionNorm (Math|Vector|Normalize (Variables|Default|GetDesiredWorldDirection))))

(fn ApplyUpRightCorrection
  (params (DeltaTime :type Float%20%28single-precision%29))
  (bind _root (Variables|Default|GetRoot))
  (bind _returnvalue (Class|MMTBPFunctionLibrary|MMTGetTransformComponent _root "Top")) ; Get transform valid during sub-stepping
  (bind _returnvalue_2 (Class|MMTBPFunctionLibrary|MMTGetTransformComponent _root "Bottom")) ; Get transform valid during sub-stepping
  (LocalVariables|SetNewDistanceToTarget (Math|Vector|VectorLength (- (+ (* (Variables|Default|GetDesiredWorldDirectionNorm) 1.1e+02) (.location _returnvalue_2)) (.location _returnvalue))))
  (Class|MMTBPFunctionLibrary|MMTAddForceatLocationComponent (Variables|Default|GetRoot) (* (- (+ (* (Variables|Default|GetDesiredWorldDirectionNorm) 1.1e+02) (.location _returnvalue_2)) (.location _returnvalue)) (- (* (Math|Vector|DotProduct (Math|Vector|Normalize (- (.location _returnvalue) (.location _returnvalue_2))) (Variables|Default|GetDesiredWorldDirection)) (Variables|Default|GetCorrectionForce)) (* (/ (- (Variables|Default|GetPreviousDistanceToTarget) (LocalVariables|GetNewDistanceToTarget)) DeltaTime) (Variables|Default|GetCorrectionDamping)))) (.location _returnvalue))
  (Variables|Default|SetPreviousDistanceToTarget (LocalVariables|GetNewDistanceToTarget)))

(fn PushinRandomDirection
  (bind _returnvalue (Math|Random|RandomFloatinRange 5e+02 8e+02))
  (bind _returnvalue_2 (Math|Random|RandomUnitVector))
  (bind _root (Variables|Default|GetRoot))
  (bind _returnvalue_3 (* _returnvalue_2 _returnvalue))
  (bind _returnvalue_4 (Transformation|GetWorldLocation _root))
  (Physics|AddImpulse (Variables|Default|GetRoot) _returnvalue_3 "None" true)
  (Rendering|Debug|DrawDebugLine _returnvalue_4 (+ _returnvalue_4 (* _returnvalue_3 0.1)) "(R=0.895000,G=0.229743,B=0.698457,A=1.000000)" 0.25 2.0))