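; Example possessable pawn demonstrating a modular drivetrain of combustion engine, dry clutch, manual gearbox and one wheel axle, with throttle, starter, clutch and shift input.
; Each physics substep passes updates from engine to wheel, resolves anisotropic friction from wheel hit contacts, then feeds the reaction back as far as the clutch.
; Tick spins or slides the part meshes and prints angular velocities, while getter functions expose drivetrain state for the possession HUD.
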(event OnComponentHit(RoadWheel)
  (params (OtherActor :type Actor%20Object%20Reference) (OtherComp :type Primitive%20Component%20Object%20Reference) (NormalImpulse :type Vector) (Hit :type Hit%20Result%20Structure%20%28by%20ref%29))
  (if (.bblockinghit Hit)
    (CallFunction|ResetFrictionPoints)
    (Default|RegisterFrictionPoint (Variables|Default|GetWheelAnisotropicFriction) "0, 0, 0" (* NormalImpulse -1.0) (.impactpoint Hit) (.impactnormal Hit))))

(event EventBeginPlay)

(event Collision|EventActorBeginOverlap
  (params (OtherActor :type Actor%20Object%20Reference)))

(event EventMMTPhysicsTick
  (params (SubstepDeltaTime :type Float%20%28single-precision%29))
  (Default|UpdatefromSourcetoApplication (Variables|Default|GetCombustionEngineModular) SubstepDeltaTime)
  (Default|UpdatefromSourcetoApplication (Variables|Default|GetDryClutchModular) SubstepDeltaTime)
  (Default|UpdatefromSourcetoApplication (Variables|Default|GetManualGearBoxModular) SubstepDeltaTime)
  (Default|UpdatefromSourcetoApplication (Variables|Default|GetWheelAxleModular) SubstepDeltaTime)
  (CallFunction|ProcessFriction SubstepDeltaTime)
  (Default|UpdatefromApplicationtoSource (Variables|Default|GetWheelAxleModular) SubstepDeltaTime)
  (Default|UpdatefromApplicationtoSource (Variables|Default|GetManualGearBoxModular) SubstepDeltaTime)
  (Default|UpdatefromApplicationtoSource (Variables|Default|GetDryClutchModular) SubstepDeltaTime))

(event EventTick
  (params (DeltaSeconds :type Float%20%28single-precision%29))
  (Variables|Default|SetIsResetFrictionPoints true)
  (Class|PrimitiveComponent|WakeAllRigidBodies (Variables|Default|GetChassis))
  (CallFunction|AnimateEngine DeltaSeconds)
  (CallFunction|AnimateClutch)
  (CallFunction|AnimateGearBoxAxles DeltaSeconds)
  (CallFunction|AnimateWheel DeltaSeconds))

(event EventPossessed
  (params (NewController :type Controller%20Object%20Reference))
  ;[1 1 1] Add and remove vehicle HUD
  (bind _asmmtcontroller (Utilities|Casting|CastToMMTController NewController))
  (Default|CreateMachineryWidget _asmmtcontroller (Variables|Default|GetHUDWidgetClass))
  (Rendering|ToggleVisibility (Variables|Default|GetHelpSign) false))

(event EventUnpossessed
  (params (OldController :type Controller%20Object%20Reference))
  ;[1 1 1] Add and remove vehicle HUD
  (bind _asmmtcontroller (Utilities|Casting|CastToMMTController OldController))
  (Default|RemoveMachineryWidget _asmmtcontroller)
  (Rendering|ToggleVisibility (Variables|Default|GetHelpSign) false))

(event Input|ActionEvents|InputActionDebugMode
  (params (Key :type Key%20Structure :default "AnyKey"))
  (:Pressed
    (Default|ToggleDebugOn/off (Variables|Default|GetPSSVisualDebugger))))

(event Input|ActionEvents|InputActionZoomIn
  (params (Key :type Key%20Structure :default "AnyKey"))
  (bind _springarm (Variables|Default|GetSpringArm))
  ;[1 1 1] Camera Control
  (:Pressed
    (Variables|/Script/Engine.SpringArmComponent|SetTargetArmLength _springarm (+ (Variables|/Script/Engine.SpringArmComponent|GetTargetArmLength _springarm) -25.0))))

(event Input|ActionEvents|InputActionZoomOut
  (params (Key :type Key%20Structure :default "AnyKey"))
  (bind _springarm (Variables|Default|GetSpringArm))
  ;[1 1 1] Camera Control
  (:Pressed
    (Variables|/Script/Engine.SpringArmComponent|SetTargetArmLength _springarm (+ (Variables|/Script/Engine.SpringArmComponent|GetTargetArmLength _springarm) 25.0))))

(event Input|AxisEvents|InputAxisVehicleForwardBackward
  (params (AxisValue :type Float%20%28single-precision%29))
  ;[1 1 1] Steering and throttle controls
  (Math|Float|CompareFloat AxisValue 0.0
    (:>
      _)
    (:==
      _))
  (Default|SetThrottle (Variables|Default|GetCombustionEngineModular) AxisValue))

(event Input|AxisEvents|InputAxisVehicleRightLeft
  (params (AxisValue :type Float%20%28single-precision%29))
  ;[1 1 1] Steering and throttle controls
  (Math|Float|CompareFloat AxisValue 0.0))

(event Input|KeyboardEvents|LeftShift
  (params (Key :type Key%20Structure :default "AnyKey"))
  (bind _dryclutchmodular (Variables|Default|GetDryClutchModular))
  ;[1 1 1] Steering and throttle controls
  (:Pressed
    (Default|PressClutch _dryclutchmodular 1.0))
  (:Released
    (Default|PressClutch _dryclutchmodular 0.0)))

(event Input|KeyboardEvents|Z
  (params (Key :type Key%20Structure :default "AnyKey"))
  ;[1 1 1] GearBox Manual Control
  (:Pressed
    (Utilities|FlowControl|Delay 0.2)
    (Default|ShiftUpDown (Variables|Default|GetManualGearBoxModular) -1)))

(event Input|KeyboardEvents|T
  (params (Key :type Key%20Structure :default "AnyKey")))

(event Input|KeyboardEvents|E
  (params (Key :type Key%20Structure :default "AnyKey"))
  (bind _combustionenginemodular (Variables|Default|GetCombustionEngineModular))
  ;[1 1 1] Steering and throttle controls
  (:Pressed
    (Default|SetStarter _combustionenginemodular true))
  (:Released
    (Default|SetStarter _combustionenginemodular false)))

(event Input|KeyboardEvents|C
  (params (Key :type Key%20Structure :default "AnyKey"))
  ;[1 1 1] GearBox Manual Control
  (:Pressed
    (Utilities|FlowControl|Delay 0.2)
    (Default|ShiftUpDown (Variables|Default|GetManualGearBoxModular) 1)))

(fn ConstructionScript
  (Rendering|Components|TextRender|SetText (Variables|Default|GetHelpSign) (Utilities|Text|MakeLiteralText "Press 4 to posses")))

(fn AnimateEngine
  (params (DeltaTime :type Float%20%28single-precision%29))
  (bind _combustionenginemodular (Variables|Default|GetCombustionEngineModular))
  (bind _angularvelocity (Variables|/Game/BluePrints/ReUsableComponents/DriveComponents/ADriveTrainComponent.ADriveTrainComponent_C|GetAngularVelocity _combustionenginemodular))
  (Transformation|AddRelativeRotation (Variables|Default|GetEngineMesh) (Math|Rotator|MakeRotator (* (Math|Trig|RadiansToDegrees _angularvelocity) DeltaTime) 0.0 0.0) false false)
  (Rendering|Debug|DrawDebugString (Transformation|GetWorldLocation (Variables|Default|GetAxleEngine)) (Utilities|String|ToString(Float) _angularvelocity) 0 "(R=1.000000,G=1.000000,B=1.000000,A=1.000000)"))

(fn AnimateClutch
  (bind _clutchplateposition (Default|GetClutchStatus (Variables|Default|GetDryClutchModular)))
  (Transformation|SetRelativeLocation (Variables|Default|GetClutchPlateLeft) (Math|Vector|MakeVector (* _clutchplateposition -5.0) 0.0 0.0) false false))

(fn AnimateGearBoxAxles
  (params (DeltaTime :type Float%20%28single-precision%29))
  (bind _manualgearboxmodular (Variables|Default|GetManualGearBoxModular))
  (bind _manualgearboxmodular_2 (Variables|Default|GetManualGearBoxModular))
  (bind _layshaftangularvelocity (Variables|/Game/BluePrints/ReUsableComponents/DriveComponents/ManualGearBoxModular.ManualGearBoxModular_C|GetLayShaftAngularVelocity _manualgearboxmodular_2))
  (bind _driveshaftangularvelocity (Variables|/Game/BluePrints/ReUsableComponents/DriveComponents/ManualGearBoxModular.ManualGearBoxModular_C|GetDriveShaftAngularVelocity _manualgearboxmodular))
  (Transformation|AddRelativeRotation (Variables|Default|GetAxleInRoot) (Math|Rotator|MakeRotator (* (Math|Trig|RadiansToDegrees _layshaftangularvelocity) DeltaTime) 0.0 0.0) false false)
  (Transformation|AddRelativeRotation (Variables|Default|GetAxleOutRoot) (Math|Rotator|MakeRotator (* (Math|Trig|RadiansToDegrees _driveshaftangularvelocity) DeltaTime) 0.0 0.0) false false)
  (Rendering|Debug|DrawDebugString (Transformation|GetWorldLocation (Variables|Default|GetAxleGearBoxIn)) (Utilities|String|ToString(Float) _layshaftangularvelocity) 0 "(R=1.000000,G=1.000000,B=1.000000,A=1.000000)")
  (Rendering|Debug|DrawDebugString (Transformation|GetWorldLocation (Variables|Default|GetAxleGearBoxOut)) (Utilities|String|ToString(Float) _driveshaftangularvelocity) 0 "(R=1.000000,G=1.000000,B=1.000000,A=1.000000)"))

(fn ProcessFriction
  (params (DeltaTime :type Float%20%28single-precision%29))
  (bind _wheelanisotropicfriction (Variables|Default|GetWheelAnisotropicFriction))
  (bind _wheelaxlemodular (Variables|Default|GetWheelAxleModular))
  (bind _isactive (Default|CheckFrictionPoint (Variables|Default|GetWheelAnisotropicFriction)))
  (if _isactive
    (Math|Integer|IncrementInt (Variables|Default|GetNumFrictionPoints)
      (:%20%20
        _)))
  (bind _driveforce (Default|GetWheelDriveForce _wheelaxlemodular))
  (bind _linearvelocity (Default|GetWheelLinearVelocity _wheelaxlemodular))
  (Default|UpdateTrackData _wheelanisotropicfriction _linearvelocity _driveforce)
  (bind _normalizedapplicationforce (Default|PhysicsUpdate _wheelanisotropicfriction (Variables|Default|GetNumFrictionPoints) DeltaTime))
  (Default|ReceiveReactionForce (Variables|Default|GetWheelAxleModular) _normalizedapplicationforce))

(fn ResetFrictionPoints
  (if (Variables|Default|GetIsResetFrictionPoints)
    (Variables|Default|SetIsResetFrictionPoints false)
    (Default|ResetFrictionPoints (Variables|Default|GetWheelAnisotropicFriction))))

(fn AnimateWheel
  (params (DeltaTIme :type Float%20%28single-precision%29))
  (bind _wheelaxlemodular (Variables|Default|GetWheelAxleModular))
  (bind _angularvelocity (Variables|/Game/BluePrints/ReUsableComponents/DriveComponents/ADriveTrainComponent.ADriveTrainComponent_C|GetAngularVelocity _wheelaxlemodular))
  (Transformation|AddLocalRotation (Variables|Default|GetRoadWheelVisual) (Math|Rotator|MakeRotator 0.0 (* (Math|Trig|RadiansToDegrees _angularvelocity) DeltaTIme -1.0) 0.0) false false)
  (Rendering|Debug|DrawDebugString (Transformation|GetWorldLocation (Variables|Default|GetWheelAxle)) (Utilities|String|ToString(Float) _angularvelocity) 0 "(R=1.000000,G=1.000000,B=1.000000,A=1.000000)"))

(fn AddDebugCoordinateSystem
  (params (DebugCoordinateSystem :type Debug%20Coordinate%20System%20Structure))
  (Default|AddDebugCoordinateSystem (Variables|Default|GetPSSVisualDebugger) DebugCoordinateSystem)
  (return false))

(fn AddDebugFloatGraph
  (params (DebugFloatGraph :type Debug%20Float%20Graph%20Input%20Structure))
  (Default|AddDebugFloatGraph (Variables|Default|GetPSSVisualDebugger) DebugFloatGraph)
  (return false))

(fn AddDebugLine
  (params (DebugLine :type Debug%20Line%20Structure))
  (Default|AddDebugLine (Variables|Default|GetPSSVisualDebugger) DebugLine)
  (return false))

(fn AddDebugString
  (params (DebugString :type Debug%20String%20Structure))
  (Default|AddDebugString (Variables|Default|GetPSSVisualDebugger) DebugString)
  (return false))

(fn HUDGetClutchStatus
  (bind _clutchstatus (Default|GetClutchStatus (Variables|Default|GetDryClutchModular)))
  (return _clutchstatus))

(fn HUDGetEngineIgnition
  (bind _inginition (Default|GetIgnition (Variables|Default|GetCombustionEngineModular)))
  (return _inginition))

(fn HUDGetEngineRPM
  (bind _enginerpm (Default|GetEngineRPMGUI (Variables|Default|GetCombustionEngineModular)))
  (return _enginerpm))

(fn HUDGetEngineRPMColor
  (bind _color (Default|GetEngineRPMColor (Variables|Default|GetCombustionEngineModular)))
  (return _color))

(fn HUDGetEngineStarter
  (bind _isstarteron (Default|GetStarterStatus (Variables|Default|GetCombustionEngineModular)))
  (return _isstarteron))

(fn HUDGetEngineTorque
  (bind _enginetorque (Default|GetEngineTorque (Variables|Default|GetCombustionEngineModular)))
  (return _enginetorque))

(fn HUDGetGearBoxInfo
  (bind (_gearnumber _isreverse) (Default|GetGearBoxInfo (Variables|Default|GetManualGearBoxModular)))
  (return _gearnumber _isreverse))

(fn HUDGetThrottle
  (bind _enginethrottle (Default|GetThrottle (Variables|Default|GetCombustionEngineModular)))
  (return _enginethrottle))

(fn HUDGetVehicleSpeed
  (return (Math|Vector|VectorLength (Transformation|GetVelocity))))