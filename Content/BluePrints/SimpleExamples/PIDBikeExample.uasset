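; Example MMT bike Blueprint that uses a PID controller to stabilize the chassis roll.
; MMTPhysicsTick updates front and back suspension stacks each substep to apply suspension forces to the chassis.
; Regular Tick feeds world roll into the PID, applies its output as torque along the chassis forward axis, and prints the signal.
; PushInRandomDirection adds random linear and angular impulses with a debug line.
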(event EventBeginPlay)

(event Collision|EventActorBeginOverlap
  (params (OtherActor :type Actor%20Object%20Reference)))

(event EventTick
  (params (DeltaSeconds :type Float%20%28single-precision%29))
  (bind _pidcontroller (Variables|Default|GetPIDController))
  (bind _chassis (Variables|Default|GetChassis))
  (Default|AddMeasuredError _pidcontroller (Utilities|Struct|MakePIDErrorStruct (.roll (Transformation|GetWorldRotation (Variables|Default|GetChassis))) DeltaSeconds))
  (bind _controlcoefficient (Default|GetControlCoefficient _pidcontroller))
  (Class|PrimitiveComponent|AddTorqueinRadians _chassis (* (Math|Vector|GetForwardVector _chassis) _controlcoefficient) "None" false)
  (Development|PrintString (Utilities|String|Append "Control signal: " (Utilities|String|ToString(Float) _controlcoefficient))))

(event EventMMTPhysicsTick
  (params (SubstepDeltaTime :type Float%20%28single-precision%29))
  ;[1 1 1] This is all what you need to apply suspension force to the "Chassis". You can see which parameters where changed from their default values in each Suspension Stack component
  (Class|MMTSuspensionStack|PhysicsUpdate (Variables|/Script/MMT.MMTSuspensionStackComponent|GetSuspensionStack (Variables|Default|GetBackSuspensionStack)) SubstepDeltaTime))

(fn ConstructionScript)

(fn PushinRandomDirection
  (bind _returnvalue (Math|Random|RandomUnitVector))
  (bind _returnvalue_2 (Math|Random|RandomFloatinRange 5e+02 8e+02))
  (bind _chassis (Variables|Default|GetChassis))
  (bind _returnvalue_3 (Transformation|GetWorldLocation _chassis))
  (bind _returnvalue_4 (* _returnvalue _returnvalue_2))
  (Physics|AddImpulse _chassis _returnvalue_4 "None" true)
  (Class|PrimitiveComponent|AddAngularImpulseinRadians (Variables|Default|GetChassis) (* (Math|Random|RandomUnitVector) (Math|Random|RandomFloatinRange 5e+04 8e+06)) "None" false)
  (Rendering|Debug|DrawDebugLine _returnvalue_3 (+ _returnvalue_3 _returnvalue_4) "(R=0.895000,G=0.229743,B=0.698457,A=1.000000)" 0.25 2.0))