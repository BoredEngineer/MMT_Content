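; Possessable MMT example vehicle demonstrating a modular drivetrain that spins physics wheels.
; Each physics substep updates engine, clutch, gearbox, differential, steering clutches and wheel axles from source to application, then back in reverse.
; Input feeds the SteeringController; Tick animates exposed drivetrain parts, plays engine and gearbox sounds and draws debug text.
; HUD getters expose drivetrain state; track friction functions exist but are never called here.
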(event EventBeginPlay
  (bind _asgear_box_51am (Utilities|Casting|CastToGearBox51AM (Components|SkeletalMesh|GetAnimInstance (Variables|Default|GetGearBox51)))
    (:then
      (Variables|Default|SetGearBoxAnimInstance _asgear_box_51am))
    (:CastFailed
      (Development|PrintString "Can't find animation instance of GearBox51" true true "(R=1.000000,G=0.000000,B=0.007700,A=1.000000)" 5.0))))

(event Collision|EventActorBeginOverlap
  (params (OtherActor :type Actor%20Object%20Reference)))

(event EventMMTPhysicsTick
  (params (SubstepDeltaTime :type Float%20%28single-precision%29))
  (Default|DTUpdatefromSourcetoApplication (Variables|Default|GetCombustionEngineModular) SubstepDeltaTime) ; >>
  (Default|DTUpdatefromSourcetoApplication (Variables|Default|GetEngineClutch) SubstepDeltaTime)
  (Default|DTUpdatefromSourcetoApplication (Variables|Default|GetManualGearBoxModular) SubstepDeltaTime)
  (Default|DTUpdatefromSourcetoApplication (Variables|Default|GetDifferentialModular) SubstepDeltaTime)
  (Default|DTUpdatefromSourcetoApplication (Variables|Default|GetRightSteeringClutch) SubstepDeltaTime)
  (Default|DTUpdatefromSourcetoApplication (Variables|Default|GetLeftSteeringClutch) SubstepDeltaTime)
  ;[1 1 1] Spinning physical wheels
  (Default|DTUpdatefromSourcetoApplication (Variables|Default|GetWheelAxleModularForRBRight) SubstepDeltaTime)
  (Default|DTUpdatefromSourcetoApplication (Variables|Default|GetWheelAxleModularForRBLeft) SubstepDeltaTime)
  (Default|DTUpdatefromApplicationtoSource (Variables|Default|GetWheelAxleModularForRBRight) SubstepDeltaTime)
  (Default|DTUpdatefromApplicationtoSource (Variables|Default|GetWheelAxleModularForRBLeft) SubstepDeltaTime)
  (Default|DTUpdatefromApplicationtoSource (Variables|Default|GetRightSteeringClutch) SubstepDeltaTime)
  (Default|DTUpdatefromApplicationtoSource (Variables|Default|GetLeftSteeringClutch) SubstepDeltaTime)
  (Default|DTUpdatefromApplicationtoSource (Variables|Default|GetDifferentialModular) SubstepDeltaTime)
  (Default|DTUpdatefromApplicationtoSource (Variables|Default|GetManualGearBoxModular) SubstepDeltaTime)
  (Default|DTUpdatefromApplicationtoSource (Variables|Default|GetEngineClutch) SubstepDeltaTime)
  (Default|DTUpdatefromApplicationtoSource (Variables|Default|GetCombustionEngineModular) SubstepDeltaTime))

(event EventPossessed
  (params (NewController :type Controller%20Object%20Reference))
  ;[1 1 1] Add and remove vehicle HUD
  (bind _asmmtcontroller (Utilities|Casting|CastToMMTController NewController))
  (Default|CreateMachineryWidget _asmmtcontroller (Variables|Default|GetHUDWidgetClass))
  (Rendering|ToggleVisibility (Variables|Default|GetHelpSign) false))

(event EventUnpossessed
  (params (OldController :type Controller%20Object%20Reference))
  ;[1 1 1] Add and remove vehicle HUD
  (bind _asmmtcontroller (Utilities|Casting|CastToMMTController OldController))
  (Default|RemoveMachineryWidget _asmmtcontroller)
  (Rendering|ToggleVisibility (Variables|Default|GetHelpSign) false))

(event EventTick
  (params (DeltaSeconds :type Float%20%28single-precision%29))
  (Variables|Default|SetIsResetFrictionPoints true)
  (Class|PrimitiveComponent|WakeAllRigidBodies (Variables|Default|GetChassis))
  (CallFunction|AnimateEngine DeltaSeconds)
  (CallFunction|AnimateClutch)
  (CallFunction|AnimateGearBoxAxles DeltaSeconds)
  (CallFunction|SteeringTest)
  (CallFunction|AnimateSteeringClutch DeltaSeconds)
  (Utilities|FlowControl|Sequence
    (:then_0
      ;[1 1 1] Play engine ignition sound
      (bind _inginition (Default|GetIgnition (Variables|Default|GetCombustionEngineModular)))
      (if _inginition
        (Utilities|FlowControl|Gate false :!label _label
          (:Exit
            (Audio|PlaySound2D "/Game/Audio/DriveTrain/EngineIgnition.EngineIgnition" 2.0 0.8)
            (Utilities|FlowControl|Sequence
              (:then_0
                (goto _label_2 Open))
              (:then_1
                (goto _label Close)))))
        (else
          (Utilities|FlowControl|Gate true :!label _label_2
            (:Exit
              (Audio|PlaySound2D "/Game/Audio/DriveTrain/EngineIgnitionOff.EngineIgnitionOff" 1.2 0.8)
              (Utilities|FlowControl|Sequence
                (:then_0
                  (goto _label Open))
                (:then_1
                  (goto _label_2 Close))))))))
    (:then_1
      ;[1 1 1] Stop playing gear box sound
      (if (Audio|Components|Audio|IsPlaying (Variables|Default|GetGearBoxClicking))
        (bind (_layshaftangularvelocity _driveshaftangularvelocity _currentgearnumber _desiredgearnumber) (Default|GetGearBoxInfo (Variables|Default|GetManualGearBoxModular)))
        (if (== _currentgearnumber _desiredgearnumber)
          (Audio|Components|Audio|Stop (Variables|Default|GetGearBoxClicking)))))))

(event Input|ActionEvents|InputActionDebugMode
  (params (Key :type Key%20Structure :default "AnyKey"))
  (:Pressed
    (Default|ToggleDebugOn/off (Variables|Default|GetPSSVisualDebugger))))

(event Input|ActionEvents|InputActionZoomIn
  (params (Key :type Key%20Structure :default "AnyKey"))
  (bind _springarm (Variables|Default|GetSpringArm))
  ;[1 1 1] Camera Control
  (:Pressed
    (Variables|/Script/Engine.SpringArmComponent|SetTargetArmLength _springarm (+ (Variables|/Script/Engine.SpringArmComponent|GetTargetArmLength _springarm) -25.0))))

(event Input|ActionEvents|InputActionZoomOut
  (params (Key :type Key%20Structure :default "AnyKey"))
  (bind _springarm (Variables|Default|GetSpringArm))
  ;[1 1 1] Camera Control
  (:Pressed
    (Variables|/Script/Engine.SpringArmComponent|SetTargetArmLength _springarm (+ (Variables|/Script/Engine.SpringArmComponent|GetTargetArmLength _springarm) 25.0))))

(event Input|AxisEvents|InputAxisVehicleForwardBackward
  (params (AxisValue :type Float%20%28single-precision%29))
  ;[1 1 1] Steering and throttle controls
  (Default|ReceiveForwardBackwardAxis (Variables|Default|GetSteeringController) AxisValue))

(event Input|AxisEvents|InputAxisVehicleRightLeft
  (params (AxisValue :type Float%20%28single-precision%29))
  ;[1 1 1] Steering and throttle controls
  (Default|ReceiveLeftRightAxis (Variables|Default|GetSteeringController) AxisValue))

(event Input|KeyboardEvents|LeftShift
  (params (Key :type Key%20Structure :default "AnyKey"))
  (bind _steeringcontroller (Variables|Default|GetSteeringController))
  ;[1 1 1] Steering and throttle controls
  (:Pressed
    (Default|ReceiveEngineClutchPedal _steeringcontroller 1.0))
  (:Released
    (Default|ReceiveEngineClutchPedal _steeringcontroller 0.0)))

(event Input|KeyboardEvents|Z
  (params (Key :type Key%20Structure :default "AnyKey"))
  (bind _gearboxclicking (Variables|Default|GetGearBoxClicking))
  ;[1 1 1] GearBox Manual Control
  (:Pressed
    (Utilities|FlowControl|Delay 0.2)
    (Default|ReceiveShiftUpDown (Variables|Default|GetSteeringController) -1)
    ;[1 1 1] Start playing clicking sound as we try to switch gear, on tick we check if gear was finally switched and stop playing sound
    (if (not (Audio|Components|Audio|IsPlaying _gearboxclicking))
      (Audio|Components|Audio|Play _gearboxclicking 0.0))))

(event Input|KeyboardEvents|E
  (params (Key :type Key%20Structure :default "AnyKey"))
  (bind _steeringcontroller (Variables|Default|GetSteeringController))
  ;[1 1 1] Steering and throttle controls
  (:Pressed
    (Default|ReceiveEngineStarter _steeringcontroller true)
    (Utilities|FlowControl|Gate false :!label _label
      (:Exit
        (Audio|PlaySound2D "/Game/Audio/DriveTrain/StarterPress.StarterPress")
        (goto _label Close))))
  (:Released
    (Default|ReceiveEngineStarter _steeringcontroller false)
    (goto _label Open)))

(event Input|KeyboardEvents|C
  (params (Key :type Key%20Structure :default "AnyKey"))
  (bind _gearboxclicking (Variables|Default|GetGearBoxClicking))
  ;[1 1 1] GearBox Manual Control
  (:Pressed
    (Utilities|FlowControl|Delay 0.2)
    (Default|ReceiveShiftUpDown (Variables|Default|GetSteeringController) 1)
    ;[1 1 1] Start playing clicking sound as we try to switch gear, on tick we check if gear was finally switched and stop playing sound
    (if (not (Audio|Components|Audio|IsPlaying _gearboxclicking))
      (Audio|Components|Audio|Play _gearboxclicking 0.0))))

(fn ConstructionScript
  (Rendering|Components|TextRender|SetText (Variables|Default|GetHelpSign) (Utilities|Text|MakeLiteralText "Press 8 to posses"))
  (CallFunction|BuildTrackSpline)
  (CallFunction|BuildTrackSpline))

(fn AnimateEngine
  (params (DeltaTime :type Float%20%28single-precision%29))
  (Utilities|FlowControl|Sequence
    (:then_0
      (bind _angularvelocity (Default|GetCrankShaftAngularVelocity (Variables|Default|GetCombustionEngineModular)))
      (Components|Timeline|SetPlayRate (Variables|Default|GetEngineAnimated) _angularvelocity)
      (Transformation|AddLocalRotation (Variables|Default|GetEngineAxlePivot) (Math|Rotator|MakeRotator (* (Math|Trig|RadiansToDegrees _angularvelocity) DeltaTime) 0.0 0.0) false false)
      (Rendering|Debug|DrawDebugString (Transformation|GetWorldLocation (Variables|Default|GetAxleEngine)) (Utilities|String|Append "Crank shaft angular velocity: 
" (Utilities|String|ToString(Float) _angularvelocity)) 0 "(R=1.000000,G=1.000000,B=1.000000,A=1.000000)"))
    (:then_1
      ;[1 1 1] Pure starter sound
      (bind _isstarteron (Default|GetStarterStatus (Variables|Default|GetCombustionEngineModular)))
      (if _isstarteron
        (if (not (Audio|Components|Audio|IsPlaying (Variables|Default|GetStarterRunning)))
          (Audio|Components|Audio|Play (Variables|Default|GetStarterRunning) 0.0))
        (else
          (Audio|Components|Audio|Stop (Variables|Default|GetStarterRunning)))))
    (:then_2
      (bind _inginition (Default|GetIgnition (Variables|Default|GetCombustionEngineModular)))
      (if _inginition
        (Utilities|FlowControl|Sequence
          (:then_0
            (if (not (Audio|Components|Audio|IsPlaying (Variables|Default|GetEngineIdle)))
              (Audio|Components|Audio|Play (Variables|Default|GetEngineIdle) 0.0)))
          (:then_1
            (if (not (Audio|Components|Audio|IsPlaying (Variables|Default|GetEngineRevving)))
              (Audio|Components|Audio|Play (Variables|Default|GetEngineRevving) 0.0)))
          (:then_2
            (bind _enginethrottle (Default|GetThrottle (Variables|Default|GetCombustionEngineModular)))
            (Audio|Components|Audio|SetVolumeMultiplier (Variables|Default|GetEngineIdle) (Math|Float|Clamp(Float) (- 1.0 (Class|KismetMathLibrary|FInterpEaseinOut 0.0 1.0 _enginethrottle 3.0)) 0.5) :!class /Script/Engine.AudioComponent)
            (Audio|Components|Audio|SetVolumeMultiplier (Variables|Default|GetEngineRevving) (Class|KismetMathLibrary|FInterpEaseinOut 0.0 1.0 _enginethrottle 3.0) :!class /Script/Engine.AudioComponent))
          (:then_3
            (bind _enginerpm (Default|GetEngineRPMGUI (Variables|Default|GetCombustionEngineModular)))
            (Audio|Components|Audio|SetPitchMultiplier (Variables|Default|GetEngineRevving) (Math|Float|MapRangeClamped _enginerpm 2.5e+02 2.1e+03 0.5 0.9))
            (Audio|Components|Audio|SetPitchMultiplier (Variables|Default|GetEngineIdle) (Math|Float|MapRangeClamped _enginerpm 2.5e+02 2.1e+03 0.5 0.9))))
        (else
          (Audio|Components|Audio|Stop (Variables|Default|GetEngineIdle))
          (Audio|Components|Audio|Stop (Variables|Default|GetEngineRevving)))))))

(fn AnimateClutch
  (bind _clutchplateposition (Default|GetClutchStatus (Variables|Default|GetEngineClutch)))
  (Transformation|SetRelativeLocation (Variables|Default|GetClutchPlateLeft) (Math|Vector|MakeVector (* _clutchplateposition -5.0) 0.0 0.0) false false))

(fn AnimateGearBoxAxles
  (params (DeltaTime :type Float%20%28single-precision%29))
  (bind (_layshaftangularvelocity _driveshaftangularvelocity _currentgearnumber _desiredgearnumber _isreverse _isgearchanging _synchroposition _synchrotarget) (Default|GetGearBoxInfo (Variables|Default|GetManualGearBoxModular)))
  (Default|SetAnimationParameters (Variables|Default|GetGearBoxAnimInstance) (* (Math|Trig|RadiansToDegrees _layshaftangularvelocity) DeltaTime) (* (Math|Trig|RadiansToDegrees _driveshaftangularvelocity) DeltaTime) _currentgearnumber _desiredgearnumber _isreverse _isgearchanging _synchroposition _synchrotarget)
  (Transformation|AddRelativeRotation (Variables|Default|GetAxleInRoot) (Math|Rotator|MakeRotator (* (Math|Trig|RadiansToDegrees _layshaftangularvelocity) DeltaTime) 0.0 0.0) false false)
  (Transformation|AddRelativeRotation (Variables|Default|GetAxleOutRoot) (Math|Rotator|MakeRotator (* (Math|Trig|RadiansToDegrees _driveshaftangularvelocity) DeltaTime) 0.0 0.0) false false)
  (Rendering|Debug|DrawDebugString (+ (Transformation|GetWorldLocation (Variables|Default|GetAxleGearBoxIn)) "0, 0,-30.000000") (Utilities|String|Append "Lay shaft angular velocity: 
" (Utilities|String|ToString(Float) _layshaftangularvelocity)) 0 "(R=0.557445,G=1.000000,B=0.804059,A=1.000000)")
  (Rendering|Debug|DrawDebugString (Transformation|GetWorldLocation (Variables|Default|GetAxleGearBoxOut)) (Utilities|String|Append "Drive shaft angular velocity: 
" (Utilities|String|ToString(Float) _driveshaftangularvelocity)) 0 "(R=0.985269,G=1.000000,B=0.988951,A=1.000000)"))

(fn ProcessFriction
  (params (DeltaTime :type Float%20%28single-precision%29))
  (LocalVariables|SetDeltaTimeLoc DeltaTime)
  (for _array_element (Utilities|Array|MakeArray 0 0 0 0 0 0 0 0 0 0 0 0)
    (bind _isactive (Default|CheckFrictionPoint _array_element))
    (if _isactive
      (Math|Integer|IncrementInt (LocalVariables|GetNumFrictionPoints))))
  (for _array_element_2 (Utilities|Array|MakeArray 0 0 0 0 0 0)
    (bind _linearvelocity (Default|GetTrackLinearVelocity (Variables|Default|GetTrackTransmissionModuleR)))
    (Default|UpdateTrackData _array_element_2 _linearvelocity)
    (bind _normalizedreactionforce (Default|PhysicsUpdate _array_element_2 (LocalVariables|GetNumFrictionPoints) (LocalVariables|GetDeltaTimeLoc)))
    (LocalVariables|SetTrackReactionForceRight (+ (LocalVariables|GetTrackReactionForceRight) _normalizedreactionforce)))
  (for _array_element_3 (Utilities|Array|MakeArray 0 0 0 0 0 0)
    (bind _linearvelocity_2 (Default|GetTrackLinearVelocity (Variables|Default|GetTrackTransmissionModuleL)))
    (Default|UpdateTrackData _array_element_3 _linearvelocity_2)
    (bind _normalizedreactionforce_2 (Default|PhysicsUpdate _array_element_3 (LocalVariables|GetNumFrictionPoints) (LocalVariables|GetDeltaTimeLoc)))
    (LocalVariables|SetTrackReactionForceLeft (+ (LocalVariables|GetTrackReactionForceLeft) _normalizedreactionforce_2)))
  (Default|ReceiveTrackReactionForce (Variables|Default|GetTrackTransmissionModuleR) (LocalVariables|GetTrackReactionForceRight))
  (Default|ReceiveTrackReactionForce (Variables|Default|GetTrackTransmissionModuleL) (LocalVariables|GetTrackReactionForceLeft))
  ;[1 1 1] Debug
  (bind _returnvalue (Class|MMTBPFunctionLibrary|MMTGetTransformComponent (Variables|Default|GetRoadWheelPhys01R) "None"))
  (CallFunction|AddDebugLine (Utilities|Struct|MakeDebugLine (.location _returnvalue) (+ (.location _returnvalue) (LocalVariables|GetTrackReactionForceRight)) "(R=0.610000,G=0.540940,B=0.000000,A=1.000000)" 0.0 5.0))
  ;[1 1 1] Debug
  (bind _returnvalue_2 (Class|MMTBPFunctionLibrary|MMTGetTransformComponent (Variables|Default|GetRoadWheelPhys01L) "None"))
  (CallFunction|AddDebugLine (Utilities|Struct|MakeDebugLine (.location _returnvalue_2) (+ (.location _returnvalue_2) (LocalVariables|GetTrackReactionForceLeft)) "(R=0.610000,G=0.540940,B=0.000000,A=1.000000)" 0.0 5.0)))

(fn ResetFrictionPoints
  (if (Variables|Default|GetIsResetFrictionPoints)
    (Variables|Default|SetIsResetFrictionPoints false)
    (Default|ResetFrictionPoints (Utilities|Array|MakeArray 0 0 0 0 0 0 0 0 0 0 0 0))))

(fn BuildTrackSpline
  (params (TrackSpline :type Spline%20Component%20Object%20Reference) (TrackAnimationDrive :type Track%20Animation%20Drive%20Object%20Reference) (TrackMesh :type Instanced%20Static%20Mesh%20Component%20Object%20Reference))
  (bind _treadsonside (Variables|/Game/BluePrints/Vehicles/Tracked/TrackComponents/TrackAnimationDrive.TrackAnimationDrive_C|GetTreadsOnSide TrackAnimationDrive))
  (Spline|SetSplinePoints TrackSpline (Variables|/Game/BluePrints/Vehicles/Tracked/TrackComponents/TrackAnimationDrive.TrackAnimationDrive_C|GetTrackSplinePointLocations TrackAnimationDrive) "Local" true)
  (for (_array_element _array_index) (Variables|/Game/BluePrints/Vehicles/Tracked/TrackComponents/TrackAnimationDrive.TrackAnimationDrive_C|GetTrackSplinePointTangents TrackAnimationDrive)
    (Spline|SetTangentatSplinePoint TrackSpline _array_index _array_element "Local" true))
  (for _index (range 0 (- _treadsonside 1))
    (Components|InstancedStaticMesh|AddInstance TrackMesh (Math|Transform|MakeTransform (Spline|GetLocationatDistanceAlongSpline TrackSpline (* _index (/ (Spline|GetSplineLength TrackSpline) (Math|Conversions|ToFloat(Integer) _treadsonside))) "Local") (Math|Rotator|MakeRotator (Math|Float|SelectFloat 1.8e+02 (.roll (Spline|GetRotationatDistanceAlongSpline TrackSpline (* _index (/ (Spline|GetSplineLength TrackSpline) (Math|Conversions|ToFloat(Integer) _treadsonside))) "Local")) (< (.y (Class|SplineComponent|GetRightVectoratDistanceAlongSpline TrackSpline (* _index (/ (Spline|GetSplineLength TrackSpline) (Math|Conversions|ToFloat(Integer) _treadsonside))) "Local")) 0.0)) (.pitch (Spline|GetRotationatDistanceAlongSpline TrackSpline (* _index (/ (Spline|GetSplineLength TrackSpline) (Math|Conversions|ToFloat(Integer) _treadsonside))) "Local")) (.yaw (Spline|GetRotationatDistanceAlongSpline TrackSpline (* _index (/ (Spline|GetSplineLength TrackSpline) (Math|Conversions|ToFloat(Integer) _treadsonside))) "Local"))) "1,1,1"))))

(fn SteeringTest
  (Utilities|FlowControl|Sequence
    (:then_0
      (bind (_clutchstatus _clutchplateposition) (Default|GetClutchStatus (Variables|Default|GetRightSteeringClutch)))
      (Rendering|Debug|DrawDebugString (Transformation|GetWorldLocation (Variables|Default|GetRoadWheelPhys01R)) (Utilities|String|Append _clutchstatus (Utilities|String|Append ": " (Utilities|String|ToString(Float) _clutchplateposition))) 0 "(R=0.000000,G=0.693872,B=1.000000,A=1.000000)"))
    (:then_1
      (bind (_clutchstatus_2 _clutchplateposition_2) (Default|GetClutchStatus (Variables|Default|GetLeftSteeringClutch)))
      (Rendering|Debug|DrawDebugString (Transformation|GetWorldLocation (Variables|Default|GetRoadWheelPhys01L)) (Utilities|String|Append _clutchstatus_2 (Utilities|String|Append ": " (Utilities|String|ToString(Float) _clutchplateposition_2))) 0 "(R=0.000000,G=0.693872,B=1.000000,A=1.000000)"))))

(fn AnimateSteeringClutch
  (params (DeltaTime :type Float%20%28single-precision%29))
  (bind _clutchplateposition (Default|GetClutchStatus (Variables|Default|GetRightSteeringClutch)))
  (Transformation|SetRelativeLocation (Variables|Default|GetInputAxleR) (Math|Vector|MakeVector (* _clutchplateposition -5.0) 0.0 0.0) false false)
  (bind _sprocketangularvelocity (Default|GetSprocketAngularVelocity (Variables|Default|GetTrackTransmissionModuleR)))
  (Transformation|AddRelativeRotation (Variables|Default|GetOutputAxleR) (Math|Rotator|MakeRotator (* (Math|Trig|RadiansToDegrees _sprocketangularvelocity) DeltaTime) 0.0 0.0) false false))

(fn AddDebugCoordinateSystem
  (params (DebugCoordinateSystem :type Debug%20Coordinate%20System%20Structure))
  (Default|AddDebugCoordinateSystem (Variables|Default|GetPSSVisualDebugger) DebugCoordinateSystem)
  (return false))

(fn AddDebugFloatGraph
  (params (DebugFloatGraph :type Debug%20Float%20Graph%20Input%20Structure))
  (Default|AddDebugFloatGraph (Variables|Default|GetPSSVisualDebugger) DebugFloatGraph)
  (return false))

(fn AddDebugLine
  (params (DebugLine :type Debug%20Line%20Structure))
  (Default|AddDebugLine (Variables|Default|GetPSSVisualDebugger) DebugLine)
  (return false))

(fn AddDebugString
  (params (DebugString :type Debug%20String%20Structure))
  (Default|AddDebugString (Variables|Default|GetPSSVisualDebugger) DebugString)
  (return false))

(fn HUDGetClutchStatus
  (bind _clutchstatus (Default|GetClutchStatus (Variables|Default|GetEngineClutch)))
  (return _clutchstatus))

(fn HUDGetEngineIgnition
  (bind _inginition (Default|GetIgnition (Variables|Default|GetCombustionEngineModular)))
  (return _inginition))

(fn HUDGetEngineRPM
  (bind _enginerpm (Default|GetEngineRPMGUI (Variables|Default|GetCombustionEngineModular)))
  (return _enginerpm))

(fn HUDGetEngineRPMColor
  (bind _color (Default|GetEngineRPMColor (Variables|Default|GetCombustionEngineModular)))
  (return _color))

(fn HUDGetEngineStarter
  (bind _isstarteron (Default|GetStarterStatus (Variables|Default|GetCombustionEngineModular)))
  (return _isstarteron))

(fn HUDGetEngineTorque
  (bind _enginetorque (Default|GetEngineTorque (Variables|Default|GetCombustionEngineModular)))
  (return _enginetorque))

(fn HUDGetGearBoxInfo
  (bind (_layshaftangularvelocity _driveshaftangularvelocity _currentgearnumber _desiredgearnumber _isreverse) (Default|GetGearBoxInfo (Variables|Default|GetManualGearBoxModular)))
  (return _currentgearnumber _desiredgearnumber _isreverse))

(fn HUDGetThrottle
  (bind _enginethrottle (Default|GetThrottle (Variables|Default|GetCombustionEngineModular)))
  (return _enginethrottle))

(fn HUDGetVehicleSpeed
  (return (Math|Vector|VectorLength (Transformation|GetVelocity))))