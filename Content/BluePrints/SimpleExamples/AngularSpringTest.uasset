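; Simple example Blueprint for testing springs, named as an angular spring test, on a physics-driven Turret.
; MMTPhysicsTick passes the substep delta time to three springs (SE, N, SW) for their physics updates.
; W and S apply a delayed vertical kick to the Turret, scaled by frame time, with downward at half strength and a debug print.
; Zoom inputs step the camera spring arm length.
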(event EventBeginPlay)

(event Collision|EventActorBeginOverlap
  (params (OtherActor :type Actor%20Object%20Reference)))

(event EventTick
  (params (DeltaSeconds :type Float%20%28single-precision%29)))

(event EventMMTPhysicsTick
  (params (SubstepDeltaTime :type Float%20%28single-precision%29))
  (Default|PhysicsUpdate (Variables|Default|GetSESpring) SubstepDeltaTime))

(event Input|ActionEvents|InputActionZoomIn
  (params (Key :type Key%20Structure :default "AnyKey"))
  (bind _springarm (Variables|Default|GetSpringArm))
  (:Pressed
    (Variables|/Script/Engine.SpringArmComponent|SetTargetArmLength _springarm (+ (Variables|/Script/Engine.SpringArmComponent|GetTargetArmLength _springarm) -25.0))))

(event Input|ActionEvents|InputActionZoomOut
  (params (Key :type Key%20Structure :default "AnyKey"))
  (bind _springarm (Variables|Default|GetSpringArm))
  (:Pressed
    (Variables|/Script/Engine.SpringArmComponent|SetTargetArmLength _springarm (+ (Variables|/Script/Engine.SpringArmComponent|GetTargetArmLength _springarm) 25.0))))

(event Input|KeyboardEvents|W
  (params (Key :type Key%20Structure :default "AnyKey"))
  (:Pressed
    (Utilities|FlowControl|Delay 0.2)
    (Physics|AddForce (Variables|Default|GetTurret) (/ (Math|Vector|MakeVector 0.0 0.0 3e+05) (Utilities|Time|GetWorldDeltaSeconds)) "None" false)
    (Development|PrintString "added Force in +Z axis" true true "(R=1.000000,G=0.000000,B=0.046095,A=1.000000)")))

(event Input|KeyboardEvents|S
  (params (Key :type Key%20Structure :default "AnyKey"))
  (:Pressed
    (Utilities|FlowControl|Delay 0.2)
    (Physics|AddForce (Variables|Default|GetTurret) (* (/ (Math|Vector|MakeVector 0.0 0.0 3e+05) (Utilities|Time|GetWorldDeltaSeconds)) -0.5) "None" false)
    (Development|PrintString "added Force in -Z axis" true true "(R=0.015103,G=1.000000,B=0.000000,A=1.000000)")))

(fn ConstructionScript)