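; Example possessable chassis that demonstrates MMT suspension and friction, with key-driven force and yaw torque, camera zoom and debug toggles.
; Each physics substep updates four suspension stacks and passes their wheel contact data to matching friction components.
; Friction components then update using the total count of active contact points.
; Random-push and slope-based reference friction helpers are defined but never called here, though Tick displays the latter's force magnitude.
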(event EventBeginPlay)

(event Collision|EventActorBeginOverlap
  (params (OtherActor :type Actor%20Object%20Reference)))

(event EventTick
  (params (DeltaSeconds :type Float%20%28single-precision%29))
  (Rendering|Debug|DrawDebugString (Transformation|GetWorldLocation (Variables|Default|GetChassis)) (Utilities|String|Append "Friction magnitude: " (Utilities|String|ToString(Float) (Variables|Default|GetFrictionForceAmplitude))) 0 "(R=1.000000,G=1.000000,B=1.000000,A=1.000000)"))

(event EventPossessed
  (params (NewController :type Controller%20Object%20Reference))
  (Rendering|ToggleVisibility (Variables|Default|GetHelpSign) false))

(event EventUnpossessed
  (params (OldController :type Controller%20Object%20Reference))
  (Rendering|ToggleVisibility (Variables|Default|GetHelpSign) false))

(event EventMMTPhysicsTick
  (params (SubstepDeltaTime :type Float%20%28single-precision%29))
  (Class|MMTSuspensionStack|PhysicsUpdate (Variables|/Script/MMT.MMTSuspensionStackComponent|GetSuspensionStack (Variables|Default|GetFrontRightSuspensionStack)) SubstepDeltaTime)
  (CallFunction|PassCollisiontoFriction (Variables|Default|GetFrontLeftFriction) (Variables|Default|GetFrontLeftSuspensionStack))
  (CallFunction|PassCollisiontoFriction (Variables|Default|GetFrontRightFriction) (Variables|Default|GetFrontRightSuspensionStack))
  (CallFunction|PassCollisiontoFriction (Variables|Default|GetBackLeftFriction) (Variables|Default|GetBackLeftSuspensionStack))
  (CallFunction|PassCollisiontoFriction (Variables|Default|GetBackRightFriction) (Variables|Default|GetBackRightSuspensionStack))
  (CallFunction|UpdateFriction SubstepDeltaTime))

(event EventMMTAfterPhysicsTick
  (params (DeltaTime :type Float%20%28single-precision%29)))

(event Input|ActionEvents|InputActionDebugMode
  (params (Key :type Key%20Structure))
  (:Pressed
    (Utilities|FlowControl|Sequence
      (:then_0
        (for _array_element (Variables|Internal|GetFrictionComponents)
          (Class|MMTFrictionComponent|ToggleDebugMode _array_element)))
      (:then_1
        (Class|MMTSuspensionStack|ToggleDebugMode (Variables|/Script/MMT.MMTSuspensionStackComponent|GetSuspensionStack (Variables|Default|GetFrontLeftSuspensionStack)))))))

(event Input|ActionEvents|InputActionZoomIn
  (params (Key :type Key%20Structure))
  (bind _springarm (Variables|Default|GetSpringArm))
  ;[1 1 1] Camera Control
  (:Pressed
    (Variables|/Script/Engine.SpringArmComponent|SetTargetArmLength _springarm (+ (Variables|/Script/Engine.SpringArmComponent|GetTargetArmLength _springarm) -25.0))))

(event Input|ActionEvents|InputActionZoomOut
  (params (Key :type Key%20Structure))
  (bind _springarm (Variables|Default|GetSpringArm))
  ;[1 1 1] Camera Control
  (:Pressed
    (Variables|/Script/Engine.SpringArmComponent|SetTargetArmLength _springarm (+ (Variables|/Script/Engine.SpringArmComponent|GetTargetArmLength _springarm) 25.0))))

(event Input|KeyboardEvents|W
  (params (Key :type Key%20Structure))
  (bind _chassis (Variables|Default|GetChassis))
  (:Pressed
    (Physics|AddForce _chassis (Math|Transform|TransformDirection (Transformation|GetWorldTransform _chassis) "20000.000000, 0,0.000000") "None" true)))

(event Input|KeyboardEvents|A
  (params (Key :type Key%20Structure))
  (bind _chassis (Variables|Default|GetChassis))
  (:Pressed
    (Class|PrimitiveComponent|AddTorqueinRadians _chassis (Math|Transform|TransformDirection (Transformation|GetWorldTransform _chassis) "0, 0,150.000000") "None" false)))

(event Input|KeyboardEvents|D
  (params (Key :type Key%20Structure))
  (bind _chassis (Variables|Default|GetChassis))
  (:Pressed
    (Class|PrimitiveComponent|AddTorqueinRadians _chassis (Math|Transform|TransformDirection (Transformation|GetWorldTransform _chassis) "0, 0,-150.000000") "None" false)))

(fn ConstructionScript
  (Variables|Internal|SetFrictionComponents (Utilities|Array|MakeArray (Variables|Default|GetFrontLeftFriction) (Variables|Default|GetFrontRightFriction) (Variables|Default|GetBackLeftFriction) (Variables|Default|GetBackRightFriction))))

(fn PushinRandomDirection
  (bind _returnvalue (Class|KismetMathLibrary|RandomUnitVectorinConeinRadians "0, 0,-1.000000" 0.523599))
  (bind _returnvalue_2 (Math|Random|RandomFloatinRange 3e+02 6e+02))
  (bind _chassis (Variables|Default|GetChassis))
  (bind _returnvalue_3 (* _returnvalue _returnvalue_2))
  (bind _returnvalue_4 (Transformation|GetWorldLocation _chassis))
  (Physics|AddImpulse _chassis _returnvalue_3 "None" true)
  (Rendering|Debug|DrawDebugLine _returnvalue_4 (+ _returnvalue_4 _returnvalue_3) "(R=0.895000,G=0.229743,B=0.698457,A=1.000000)" 0.25 2.0))

(fn PassCollisiontoFriction
  (params (FrictionComponent :type MMT%20Friction%20Component%20Object%20Reference) (SuspensionStack :type MMT%20Suspension%20Stack%20Component%20Object%20Reference))
  ;[1 1 1] When suspension stack finds location for the wheel, it records data about where wheel would collide with the ground.
  ; This collision data is passed to friction component to calculate friction force.
  (bind (_bpointactive _forceatpoint _pointlocation _surfacenormal _surfacephysicalmaterial _surfacevelocity) (Class|MMTSuspensionStack|GetContactData (Variables|/Script/MMT.MMTSuspensionStackComponent|GetSuspensionStack SuspensionStack)))
  (Class|MMTFrictionComponent|ResetFrictionPoints FrictionComponent)
  (if _bpointactive
    (Class|MMTFrictionComponent|RegisterFrictionPoint FrictionComponent _forceatpoint false _pointlocation _surfacenormal _surfacephysicalmaterial _surfacevelocity)))

(fn UpdateFriction
  (params (DeltaTime :type Float%20%28single-precision%29))
  (LocalVariables|SetDT DeltaTime)
  ;[1 1 1] First we need to count total amount of friction points that need to be processed. Friction point is counted as active if it received
  ; a valid contact point information, from another component, such as suspension stack.
  (for _array_element (Variables|Internal|GetFrictionComponents)
    (bind _returnvalue (Class|MMTFrictionComponent|IsFrictionPointActive _array_element))
    (if _returnvalue
      (Math|Integer|IncrementInt (LocalVariables|GetPointsCount))))
  (Class|MMTFrictionComponent|PhysicsUpdate (Variables|Default|GetFrontLeftFriction) (Math|Conversions|ToFloat(Integer) (LocalVariables|GetPointsCount)) (LocalVariables|GetDT))
  (Class|MMTFrictionComponent|PhysicsUpdate (Variables|Default|GetFrontRightFriction) (Math|Conversions|ToFloat(Integer) (LocalVariables|GetPointsCount)) (LocalVariables|GetDT))
  (Class|MMTFrictionComponent|PhysicsUpdate (Variables|Default|GetBackLeftFriction) (Math|Conversions|ToFloat(Integer) (LocalVariables|GetPointsCount)) (LocalVariables|GetDT))
  (Class|MMTFrictionComponent|PhysicsUpdate (Variables|Default|GetBackRightFriction) (Math|Conversions|ToFloat(Integer) (LocalVariables|GetPointsCount)) (LocalVariables|GetDT)))

(fn ComputeandApplyReferenceFriction
  (params (DeltaTime :type Float%20%28single-precision%29))
  (bind _chassis (Variables|Default|GetChassis))
  (bind _chassis_2 (Variables|Default|GetChassis))
  (bind _chassis_3 (Variables|Default|GetChassis))
  (bind _chassis_4 (Variables|Default|GetChassis))
  (bind _returnvalue (Transformation|GetWorldLocation _chassis_2))
  (bind _returnvalue_2 (Physics|GetMass _chassis))
  (bind _returnvalue_3 (Transformation|GetWorldLocation _chassis_3))
  (bind _returnvalue_4 (* _returnvalue_2 9.8e+02))
  (LocalVariables|SetDT DeltaTime)
  (bind _outhit (Collision|LineTraceByChannel _returnvalue_3 (+ _returnvalue_3 (* (Math|Vector|GetUpVector _chassis_3) -1e+02)) "TraceTypeQuery1" false 0 "ForOneFrame"))
  (if (.bblockinghit _outhit)
    (LocalVariables|SetImpactNormal (.impactnormal _outhit))
    (LocalVariables|SetFrictionDirection (Math|Vector|Normalize (Math|Vector|ProjectVectorontoPlane "0, 0,1.000000" (.impactnormal _outhit))))
    (LocalVariables|SetCosA (Math|Vector|DotProduct (LocalVariables|GetFrictionDirection) (Math|Vector|Normalize (Math|Vector|MakeVector (.X (Math|Vector|BreakVector (LocalVariables|GetFrictionDirection))) (.Y (Math|Vector|BreakVector (LocalVariables|GetFrictionDirection))) 0.0))))
    (Rendering|Debug|DrawDebugString (+ (Transformation|GetWorldLocation _chassis_4) (* (Math|Vector|GetUpVector _chassis_4) 1e+02)) (Utilities|String|Append "Slope angle: " (Utilities|String|ToString(Float) (Class|KismetMathLibrary|DegAtan2 (Math|Vector|VectorLength (Math|Vector|CrossProduct (LocalVariables|GetFrictionDirection) (Math|Vector|Normalize (Math|Vector|MakeVector (.X (Math|Vector|BreakVector (LocalVariables|GetFrictionDirection))) (.Y (Math|Vector|BreakVector (LocalVariables|GetFrictionDirection))) 0.0)))) (Math|Vector|DotProduct (LocalVariables|GetFrictionDirection) (Math|Vector|Normalize (Math|Vector|MakeVector (.X (Math|Vector|BreakVector (LocalVariables|GetFrictionDirection))) (.Y (Math|Vector|BreakVector (LocalVariables|GetFrictionDirection))) 0.0)))))) 0 "(R=1.000000,G=1.000000,B=1.000000,A=1.000000)")
    (LocalVariables|SetSinA (Math|Trig|Sin(Degrees) (Class|KismetMathLibrary|DegAtan2 (Math|Vector|VectorLength (Math|Vector|CrossProduct (LocalVariables|GetFrictionDirection) (Math|Vector|Normalize (Math|Vector|MakeVector (.X (Math|Vector|BreakVector (LocalVariables|GetFrictionDirection))) (.Y (Math|Vector|BreakVector (LocalVariables|GetFrictionDirection))) 0.0)))) (Math|Vector|DotProduct (LocalVariables|GetFrictionDirection) (Math|Vector|Normalize (Math|Vector|MakeVector (.X (Math|Vector|BreakVector (LocalVariables|GetFrictionDirection))) (.Y (Math|Vector|BreakVector (LocalVariables|GetFrictionDirection))) 0.0))))))
    (bind _output_get (LocalVariables|SetFrictionForceAmplitudeLoc (* _returnvalue_4 (LocalVariables|GetSinA))))
    (if (and (!= _output_get 0.0) (<= _output_get (* _returnvalue_4 (* (LocalVariables|GetCosA) (Variables|Default|GetFrictionCoefficient)))))
      (Variables|Default|SetFrictionForceAmplitude (LocalVariables|GetFrictionForceAmplitudeLoc))
      (Class|MMTBPFunctionLibrary|MMTAddForceComponent (Variables|Default|GetChassis) (* (LocalVariables|GetFrictionDirection) (LocalVariables|GetFrictionForceAmplitudeLoc)) false)
      (Rendering|Debug|DrawDebugLine _returnvalue (+ _returnvalue (* (LocalVariables|GetFrictionDirection) (LocalVariables|GetFrictionForceAmplitudeLoc))) "(R=1.000000,G=0.055000,B=0.671518,A=1.000000)" 0.0 5.0))))