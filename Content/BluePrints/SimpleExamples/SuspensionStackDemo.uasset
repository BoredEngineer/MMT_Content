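; Example Blueprint that demonstrates suspension forces on a Chassis using four Suspension Stack components, one per corner.
; The MMT physics tick passes the substep delta time to each stack's PhysicsUpdate, which is all the suspension needs.
; A PushInRandomDirection function jolts the chassis with a random velocity-change impulse and draws a brief debug line, randomized separately from that impulse.
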(event EventBeginPlay)

(event Collision|EventActorBeginOverlap
  (params (OtherActor :type Actor%20Object%20Reference)))

(event EventTick
  (params (DeltaSeconds :type Float%20%28single-precision%29)))

(event EventMMTPhysicsTick
  (params (SubstepDeltaTime :type Float%20%28single-precision%29))
  ;[1 1 1] This is all what you need to apply suspension force to the "Chassis". You can see which parameters where changed from their default values in each Suspension Stack component
  (Class|MMTSuspensionStack|PhysicsUpdate (Variables|/Script/MMT.MMTSuspensionStackComponent|GetSuspensionStack (Variables|Default|GetFrontRightSuspensionStack)) SubstepDeltaTime))

(fn ConstructionScript)

(fn PushinRandomDirection
  (bind _returnvalue (Math|Random|RandomFloatinRange 5e+02 8e+02))
  (bind _returnvalue_2 (Math|Random|RandomUnitVector))
  (bind _chassis (Variables|Default|GetChassis))
  (bind _returnvalue_3 (* _returnvalue_2 _returnvalue))
  (bind _returnvalue_4 (Transformation|GetWorldLocation _chassis))
  (Physics|AddImpulse _chassis _returnvalue_3 "None" true)
  (Rendering|Debug|DrawDebugLine _returnvalue_4 (+ _returnvalue_4 _returnvalue_3) "(R=0.895000,G=0.229743,B=0.698457,A=1.000000)" 0.25 2.0))