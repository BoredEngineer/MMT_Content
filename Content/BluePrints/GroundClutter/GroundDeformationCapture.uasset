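; Scene-capture actor that follows a tracking target from a height offset to feed ground deformation on the landscape.
; Capture width comes from FOV and Z offset, and world texel size from that width and render target resolution.
; Each tick it snaps its position to the texel grid once the target moves over a texel.
; It writes capture size and position to the LandscapeParams material parameter collection for projecting the texture.
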(event EventBeginPlay
  (CallFunction|CalculateSize)
  (CallFunction|CalculateTexelSize)
  (CallFunction|UpdateMaterialParametersCaptureSize))

(event Collision|EventActorBeginOverlap
  (params (OtherActor :type Actor%20Object%20Reference)))

(event EventTick
  (params (DeltaSeconds :type Float%20%28single-precision%29))
  (CallFunction|FollowTarget)
  (CallFunction|UpdateMaterialParametersTrackerPosition))

(fn ConstructionScript
  (CallFunction|CalculateSize)
  (CallFunction|CalculateTexelSize)
  (CallFunction|FollowTarget)
  (CallFunction|UpdateMaterialParametersCaptureSize)
  (CallFunction|UpdateMaterialParametersTrackerPosition))

(fn CalculateSize
  ;[1 1 1] Find size of the scene capture by using calculation rules of right triangle. Camera frustum can be split
  ; verticaly into two right triangles. We know length of adjucent side and angle, then opposite is:
  ; opposite = adjacent * tan(a)
  (Variables|Default|SetCaptureSize (* (Math|Trig|Tan(Degrees) (/ (Variables|/Script/Engine.SceneCaptureComponent2D|GetFOVAngle (Variables|Default|GetSceneCaptureComponent2D)) 2.0)) (Variables|Default|GetZOffset) 2.0)))

(fn CalculateTexelSize
  (bind _scenecapturecomponent2d (Variables|Default|GetSceneCaptureComponent2D))
  (bind _texturetarget (Variables|/Script/Engine.SceneCaptureComponent2D|GetTextureTarget _scenecapturecomponent2d))
  ;[1 1 1] We calculate size of the SceneCapture texel in world space, to later use it for snapping position of the SceneCapture to a grid
  (Variables|Default|SetTexelSizeX (* (/ (Variables|Default|GetCaptureSize) (Math|Conversions|ToFloat(Integer) (Variables|/Script/Engine.TextureRenderTarget2D|GetSizeX _texturetarget))) (Variables|Default|GetTexelSizeMult)))
  (Variables|Default|SetTexelSizeY (* (/ (Variables|Default|GetCaptureSize) (Math|Conversions|ToFloat(Integer) (Variables|/Script/Engine.TextureRenderTarget2D|GetSizeY _texturetarget))) (Variables|Default|GetTexelSizeMult))))

(fn UpdateMaterialParametersCaptureSize
  (bind _capturesize (Variables|Default|GetCaptureSize))
  (Rendering|Material|SetVectorParameterValue "/Game/Materials/Maps/LandscapeParams.LandscapeParams" "TextureSize" (Math|Conversions|ToLinearColor(Vector) (Math|Vector|MakeVector _capturesize _capturesize _capturesize)) :!class /Script/Engine.KismetMaterialLibrary))

(fn UpdateMaterialParametersTrackerPosition
  (Rendering|Material|SetVectorParameterValue "/Game/Materials/Maps/LandscapeParams.LandscapeParams" "TrackerPosition" (Math|Conversions|ToLinearColor(Vector) (Transformation|GetActorLocation)) :!class /Script/Engine.KismetMaterialLibrary))

(fn FollowTarget
  (bind _trackingtarget (Variables|Default|GetTrackingTarget))
  (bind _texelsizey (Variables|Default|GetTexelSizeY))
  (bind _texelsizex (Variables|Default|GetTexelSizeX))
  (bind _returnvalue (Transformation|GetActorLocation _trackingtarget))
  (bind _returnvalue_2 (Math|Float|Min(Float) _texelsizex _texelsizey))
  (if (and (Utilities|IsValid (Variables|Default|GetTrackingTarget)) (> (Math|Vector|VectorLength (- (Transformation|GetActorLocation (Variables|Default|GetTrackingTarget)) (Variables|Default|GetPreviousCoordinates))) (Math|Float|Min(Float) (Variables|Default|GetTexelSizeX) (Variables|Default|GetTexelSizeY))))
    ;[1 1 1] We "snap" position of ScenCapture to discrete grid, corelated with size of the texture projected on landscape in world space
    (Transformation|SetActorLocation (Math|Vector|MakeVector (* (.ReturnValue (Math|Float|Division(WholeandRemainder) (.x _returnvalue) (Variables|Default|GetTexelSizeX))) (Variables|Default|GetTexelSizeX)) (* (.ReturnValue (Math|Float|Division(WholeandRemainder) (.y _returnvalue) (Variables|Default|GetTexelSizeY))) (Variables|Default|GetTexelSizeY)) (* (.ReturnValue (Math|Float|Division(WholeandRemainder) (+ (+ (.z _returnvalue) (Variables|Default|GetLandscapeCaptureOffset)) (Variables|Default|GetZOffset)) _returnvalue_2)) _returnvalue_2)) false false)
    (Variables|Default|SetPreviousCoordinates (Transformation|GetActorLocation (Variables|Default|GetTrackingTarget)))))

(fn GetMaterialParameters
  (bind _capturesize (Variables|Default|GetCaptureSize))
  (return (Math|Vector|MakeVector _capturesize _capturesize _capturesize) (Transformation|GetActorLocation)))