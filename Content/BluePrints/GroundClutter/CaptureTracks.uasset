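; CaptureTracks is a scene capture actor that follows a tracking target and feeds its position and coverage to landscape material parameters, apparently for ground tracks.
; Construction derives capture width from camera FOV and height offset, then texel size from the render target resolution.
; Each tick it snaps its location to that texel grid around the target and writes position and size into the LandscapeParams parameter collection.
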(event EventBeginPlay)

(event EventTick
  (params (DeltaSeconds :type Float%20%28single-precision%29))
  (CallFunction|FollowTarget)
  (CallFunction|UpdateParameters))

(fn ConstructionScript
  (CallFunction|CalculateSize)
  (CallFunction|FollowTarget)
  (CallFunction|UpdateParameters))

(fn FollowTarget
  (bind _texelsizex (Variables|Default|GetTexelSizeX))
  (bind _texelsizey (Variables|Default|GetTexelSizeY))
  (bind _trackingtarget (Variables|Default|GetTrackingTarget))
  (bind _returnvalue (Transformation|GetActorLocation _trackingtarget))
  (bind _returnvalue_2 (Math|Float|Max(Float) _texelsizex _texelsizey))
  (Utilities|IsValid (Variables|Default|GetTrackingTarget)
    (:Is%20Valid
      ;[1 1 1] We "snap" position of ScenCapture to discrete grid, corelated with size of the texture projected on landscape
      ; in world space
      (Transformation|SetActorLocation (Math|Vector|MakeVector (* (.ReturnValue (Math|Float|Division(WholeandRemainder) (.x _returnvalue) (Variables|Default|GetTexelSizeX))) (Variables|Default|GetTexelSizeX)) (* (.ReturnValue (Math|Float|Division(WholeandRemainder) (.y _returnvalue) (Variables|Default|GetTexelSizeY))) (Variables|Default|GetTexelSizeY)) (* (.ReturnValue (Math|Float|Division(WholeandRemainder) (+ (- (.z _returnvalue) (Variables|Default|GetLandscapeCaptureOffset)) (Variables|Default|GetZOffset)) _returnvalue_2)) _returnvalue_2)) false false))))

(fn UpdateParameters
  (bind _capturesize (Variables|Default|GetCaptureSize))
  (Rendering|Material|SetVectorParameterValue "/Game/Materials/Maps/LandscapeParams.LandscapeParams" "TrackerPosition" (Math|Conversions|ToLinearColor(Vector) (Transformation|GetActorLocation)) :!class /Script/Engine.KismetMaterialLibrary)
  (Rendering|Material|SetVectorParameterValue "/Game/Materials/Maps/LandscapeParams.LandscapeParams" "TextureSize" (Math|Conversions|ToLinearColor(Vector) (Math|Vector|MakeVector _capturesize _capturesize _capturesize)) :!class /Script/Engine.KismetMaterialLibrary))

(fn CalculateSize
  (bind _capturecomponent2d (Variables|DecalActor|GetCaptureComponent2D))
  (bind _texturetarget (Variables|/Script/Engine.SceneCaptureComponent2D|GetTextureTarget _capturecomponent2d))
  ;[1 1 1] Find size of the scene capture by using calculation rules of right triangle. Camera frustum can be split
  ; verticaly into two right triangles. We know length of adjucent side and angle, then opposite is:
  ; opposite = adjacent * tan(a)
  (Variables|Default|SetCaptureSize (* (Math|Trig|Tan(Degrees) (/ (Variables|/Script/Engine.SceneCaptureComponent2D|GetFOVAngle (Variables|DecalActor|GetCaptureComponent2D)) 2.0)) (Variables|Default|GetZOffset) 2.0))
  (Variables|Default|SetTexelSizeX (/ (Variables|Default|GetCaptureSize) (Math|Conversions|ToFloat(Integer) (Variables|/Script/Engine.TextureRenderTarget2D|GetSizeX _texturetarget))))
  (Variables|Default|SetTexelSizeY (/ (Variables|Default|GetCaptureSize) (Math|Conversions|ToFloat(Integer) (Variables|/Script/Engine.TextureRenderTarget2D|GetSizeY _texturetarget)))))